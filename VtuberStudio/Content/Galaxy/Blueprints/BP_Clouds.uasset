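; BP_Clouds is a galaxy cloud effect actor that pairs a Niagara system with a point light.
; Its construction script applies the actor's intensity, attenuation radius and colour variables to the light.
; It also feeds drag, cloud disk radius and a static mesh override into the Niagara User parameters.
; The event graph holds only disabled stub events, so the Blueprint has no runtime logic.
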(event EventBeginPlay)

(event Collision|EventActorBeginOverlap
  (params (OtherActor :type Actor%20Object%20Reference)))

(event EventTick
  (params (DeltaSeconds :type Float%20%28single-precision%29)))

(fn ConstructionScript
  (bind _pointlight (Variables|Default|GetPointLight))
  (bind _niagara (Variables|Default|GetNiagara))
  (Rendering|Components|Light|SetIntensity _pointlight (Variables|PointLight|GetLight%20Intensity))
  (Rendering|Lighting|SetAttenuationRadius _pointlight (Variables|PointLight|GetAttenuation%20Radius))
  (Rendering|Components|Light|SetLightColor _pointlight (Variables|PointLight|GetPointLightColour) true)
  (Niagara|SetNiagaraVariable(Float) _niagara "User.Drag" (Variables|Clouds|GetDrag))
  (Class|NiagaraFunctionLibrary|OverrideSystemUserVariableStaticMesh _niagara "User.Mesh" (Variables|Clouds|GetStatic%20Mesh))
  (Niagara|SetNiagaraVariable(Float) _niagara "User.CloudDiskRadius" (Variables|Clouds|GetCloudDiskRadius)))