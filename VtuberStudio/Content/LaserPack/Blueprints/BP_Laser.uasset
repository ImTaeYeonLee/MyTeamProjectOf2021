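; BP_Laser is a laser actor that shows a colored beam along its arrow, cut short at the first blocking object.
; At game start, Beam traces on Visibility up to the beam length, and CreateBeam spawns the particle system that GetColor picks for the selected color.
; Each tick repeats the trace and moves the existing emitter and its beam end point rather than respawning it.
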(event Custom|CustomEvent
  (params (DeltaSeconds :type Float%20%28single-precision%29))
  (bind _emietter (Variables|Default|GetEmietter))
  (bind _arrow (Variables|Default|GetArrow))
  (bind _beam_lenght (Variables|Options|GetBeam%20lenght))
  (bind _returnvalue (Math|Float|MakeLiteralFloat _beam_lenght))
  (bind _returnvalue_2 (Transformation|GetWorldLocation _arrow))
  (bind _returnvalue_3 (Transformation|GetWorldRotation _arrow))
  (bind _returnvalue_4 (Math|Rotator|GetRotationXVector _returnvalue_3))
  (bind _returnvalue_5 (* _returnvalue_4 _returnvalue))
  (bind _returnvalue_6 (+ _returnvalue_2 _returnvalue_5))
  ;[1 1 1] Each tick, re-calculate the laser
  (Variables|Default|SetBeam%20end%20point _returnvalue_6)
  ;;[1 1 1] Detect if there is any object blocking the way
  (bind (_outhit _returnvalue_7) (Collision|LineTraceByChannel _returnvalue_2 _returnvalue_6 "TraceTypeQuery1" true 0 "None"))
  (if _returnvalue_7
    (bind _output_get (Variables|Default|SetBeam%20end%20point (.ImpactPoint (Collision|BreakHitResult _outhit)))))
  ;;[1 1 1] Set the new beam
  (Class|ParticleSystemComponent|SetBeamEndPoint _emietter 0 _output_get)
  (Transformation|SetWorldLocation _emietter _returnvalue_2 false false))

(event Custom|CustomEvent_1
  ;[1 1 1] Create the beam at the start of the game
  ;;[1 1 1] This Function Generate the beam
  (CallFunction|Beam))

(fn ConstructionScript)

(fn CreateBeam
  (params (Start :type Vector) (End :type Vector))
  ;[1 1 1] If the beam exist already, delete the previous beam
  (Utilities|IsValid (Variables|Default|GetEmietter)
    (:Is%20Valid
      (Components|DestroyComponent (Variables|Default|GetEmietter)))
    (:Is%20Not%20Valid
      _))
  ;[1 1 1] Use this function to get the particle system corresponding to the selected color
  (bind _out (CallFunction|GetColor (Variables|Options|GetColor)))
  ;[1 1 1] Create the laser
  (bind _returnvalue (Effects|SpawnEmitteratLocation _out Start))
  ;[1 1 1] Set the end point
  (bind _output_get (Variables|Default|SetEmietter _returnvalue))
  (Class|ParticleSystemComponent|SetBeamEndPoint _output_get 0 End))

(fn GetColor
  (params (Color :type Colors%20Enum :default "NewEnumerator0"))
  ;[1 1 1] Depending on the selected color, output the corresponding laser particle system
  (switch Utilities|FlowControl|Switch|SwitchonColors Color
    (:NewEnumerator0
      (return "/Game/LaserPack/Particles/Laser_Blue.Laser_Blue"))
    (:NewEnumerator1
      (return "/Game/LaserPack/Particles/Laser_LightBlue.Laser_LightBlue"))
    (:NewEnumerator2
      (return "/Game/LaserPack/Particles/Laser_Purple.Laser_Purple"))
    (:NewEnumerator3
      (return "/Game/LaserPack/Particles/Laser_Red.Laser_Red"))
    (:NewEnumerator4
      (return "/Game/LaserPack/Particles/Laser_Pink.Laser_Pink"))
    (:NewEnumerator5
      (return "/Game/LaserPack/Particles/Laser_Orange.Laser_Orange"))
    (:NewEnumerator6
      (return "/Game/LaserPack/Particles/Laser_Yellow.Laser_Yellow"))
    (:NewEnumerator7
      (return "/Game/LaserPack/Particles/Laser_Green.Laser_Green"))
    (:NewEnumerator8
      (return "/Game/LaserPack/Particles/Laser_White.Laser_White"))
    (:NewEnumerator9
      (return "/Game/LaserPack/Particles/Laser_Off.Laser_Off"))))

(fn Beam
  (bind _arrow (Variables|Default|GetArrow))
  (bind _beam_lenght (Variables|Options|GetBeam%20lenght))
  (bind _returnvalue (Math|Float|MakeLiteralFloat _beam_lenght))
  (bind _returnvalue_2 (Transformation|GetWorldLocation _arrow))
  (bind _returnvalue_3 (Transformation|GetWorldRotation _arrow))
  (bind _returnvalue_4 (Math|Rotator|GetRotationXVector _returnvalue_3))
  (bind _returnvalue_5 (* _returnvalue_4 _returnvalue))
  (bind _returnvalue_6 (+ _returnvalue_2 _returnvalue_5))
  ;[1 1 1] Create a simple beam
  (Variables|Default|SetBeam%20end%20point _returnvalue_6)
  ;;[1 1 1] Check if there is an object blocking the way
  (bind (_outhit _returnvalue_7) (Collision|LineTraceByChannel _returnvalue_2 _returnvalue_6 "TraceTypeQuery1" true 0 "None"))
  (if _returnvalue_7
    ;;[1 1 1] If hit, set the end point to the hit location
    (bind _output_get (Variables|Default|SetBeam%20end%20point (.ImpactPoint (Collision|BreakHitResult _outhit)))))
  ;;[1 1 1] Use this function to create the beam according to the start and the end point
  (CallFunction|CreateBeam (Transformation|GetWorldLocation (Variables|Default|GetArrow)) _output_get))