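; BP_LaserMultiBox is a laser box that fires one timed beam at a time from five arrow components in sequence.
; An endless BeginPlay loop line-traces along the current arrow to clip the beam at obstacles, then spawns a beam particle in the selected or random color.
; After the on-time it destroys the emitter, steps to the next arrow, wrapping or ping-ponging by Mode, and waits before firing again.
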(event EventBeginPlay
  (bind _emietter (Variables|Components|GetEmietter))
  ;[1 1 1] At the start of the game, add all the arrows to an array
  (|AddToArray)
  ;[1 1 1] Create a beam out of the specified arrow
  ;;[1 1 1] Detect if there is any object blocking the way
  (bind (_outhit _returnvalue) (Collision|LineTraceByChannel (Transformation|GetWorldLocation (Utilities|Array|Get(acopy) (Variables|Default|GetArrows) (Variables|Default|GetBeamNumber))) (+ (Transformation|GetWorldLocation (Utilities|Array|Get(acopy) (Variables|Default|GetArrows) (Variables|Default|GetBeamNumber))) (* (Math|Rotator|GetRotationXVector (Transformation|GetWorldRotation (Utilities|Array|Get(acopy) (Variables|Default|GetArrows) (Variables|Default|GetBeamNumber)))) (Math|Float|MakeLiteralFloat (Variables|Options|GetBeam%20lenght)))) "TraceTypeQuery1" true 0 "None" :!label _label))
  (if _returnvalue
    ;;[1 1 1] If hit, set the end point to the hit location
    (Variables|Default|SetBeam%20end%20point (.ImpactPoint (Collision|BreakHitResult _outhit)))
    (else
      (Variables|Default|SetBeam%20end%20point (+ (Transformation|GetWorldLocation (Utilities|Array|Get(acopy) (Variables|Default|GetArrows) (Variables|Default|GetBeamNumber))) (* (Math|Rotator|GetRotationXVector (Transformation|GetWorldRotation (Utilities|Array|Get(acopy) (Variables|Default|GetArrows) (Variables|Default|GetBeamNumber)))) (Math|Float|MakeLiteralFloat (Variables|Options|GetBeam%20lenght)))))))
  ;;[1 1 1] Use this function to create the beam according to the defined start and end location
  (CallFunction|CreateBeam (Transformation|GetWorldLocation (Utilities|Array|Get(acopy) (Variables|Default|GetArrows) (Variables|Default|GetBeamNumber))) (Variables|Default|GetBeam%20end%20point) false)
  (Utilities|FlowControl|Delay (Variables|Options|GetTime%20ON))
  (Utilities|IsValid _emietter
    (:Is%20Valid
      (Components|DestroyComponent _emietter))
    (:Is%20Not%20Valid
      _))
  ;[1 1 1] Select the next arrow
  (if (Variables|Default|GetInc?)
    (if (== (Variables|Default|GetBeamNumber) 4)
      (if (Utilities|Enum|Equal(Enum) (Variables|Options|GetMode) "NewEnumerator1")
        (Variables|Default|SetInc? false)
        (bind _result (Math|Integer|DecrementInt (Variables|Default|GetBeamNumber))
          (:%20%20
            (Variables|Default|SetBeamNumber _result)))
        (else
          (Variables|Default|SetBeamNumber 0)))
      (else
        (bind _result_2 (Math|Integer|IncrementInt (Variables|Default|GetBeamNumber))
          (:%20%20
            (Variables|Default|SetBeamNumber _result_2)))))
    (elif (== (Variables|Default|GetBeamNumber) 0)
      (bind _result_3 (Math|Integer|IncrementInt (Variables|Default|GetBeamNumber))
        (:%20%20
          (Variables|Default|SetBeamNumber _result_3)
          (Variables|Default|SetInc? true)))
      (else
        (bind _result_4 (Math|Integer|DecrementInt (Variables|Default|GetBeamNumber))
          (:%20%20
            (Variables|Default|SetBeamNumber _result_4))))))
  (Utilities|FlowControl|Delay (Variables|Options|GetDelayBetweenLasers))
  (goto _label))

(fn ConstructionScript)

(fn CreateBeam
  (params (Start :type Vector) (End :type Vector) (Destroy%20? :type Boolean))
  ;[1 1 1] If the beam exist already, delete the previous beam
  (Utilities|IsValid (Variables|Components|GetEmietter)
    (:Is%20Valid
      (Components|DestroyComponent (Variables|Components|GetEmietter)))
    (:Is%20Not%20Valid
      _))
  ;[1 1 1] If random color mode is selected, set the color to a random one
  (if (Variables|Options|GetRandom%20Colors%20?)
    (|SelectRandomColor))
  (bind _out (CallFunction|GetColor (Variables|Options|GetColor)))
  ;[1 1 1] Create the particle
  (bind _returnvalue (Effects|SpawnEmitteratLocation _out Start "0, 0, 0" "1.000000,1.000000,1.000000" Destroy%20?))
  (bind _output_get (Variables|Components|SetEmietter _returnvalue))
  (Class|ParticleSystemComponent|SetBeamEndPoint _output_get 0 End))

(fn GetColor
  (params (Color :type Colors%20Enum :default "NewEnumerator0"))
  ;[1 1 1] Depending on the selected color, output the corresponding laser particle system
  (switch Utilities|FlowControl|Switch|SwitchonColors Color
    (:NewEnumerator0
      (return "/Game/LaserPack/Particles/Laser_Blue.Laser_Blue"))
    (:NewEnumerator1
      (return "/Game/LaserPack/Particles/Laser_LightBlue.Laser_LightBlue"))
    (:NewEnumerator2
      (return "/Game/LaserPack/Particles/Laser_Purple.Laser_Purple"))
    (:NewEnumerator3
      (return "/Game/LaserPack/Particles/Laser_Red.Laser_Red"))
    (:NewEnumerator4
      (return "/Game/LaserPack/Particles/Laser_Pink.Laser_Pink"))
    (:NewEnumerator5
      (return "/Game/LaserPack/Particles/Laser_Orange.Laser_Orange"))
    (:NewEnumerator6
      (return "/Game/LaserPack/Particles/Laser_Yellow.Laser_Yellow"))
    (:NewEnumerator7
      (return "/Game/LaserPack/Particles/Laser_Green.Laser_Green"))
    (:NewEnumerator8
      (return "/Game/LaserPack/Particles/Laser_White.Laser_White"))
    (:NewEnumerator9
      (return "/Game/LaserPack/Particles/Laser_Off.Laser_Off"))))