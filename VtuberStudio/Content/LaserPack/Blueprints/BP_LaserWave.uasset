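; BP_LaserWave is a laser effect actor that fires a set of colored beams from six arrow components.
; On BeginPlay it gathers the arrows into an array and line traces along each forward vector up to BeamLenght, ending the beam at any visibility hit.
; CreateBeam spawns the particle system that GetColor picks for the selected color and sets its beam end point.
; Beams are computed only once, with no later updates.
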(event EventBeginPlay
  ;[1 1 1] Add all the arrows to an array
  (|AddToArrows)
  ;[1 1 1] Loot all the arrows and create a beam out of them
  (for _array_element (Variables|Default|GetArrows)
    ;;[1 1 1] Detect if there is any object blocking the way
    (bind (_outhit _returnvalue) (Collision|LineTraceByChannel (Transformation|GetWorldLocation _array_element) (+ (Transformation|GetWorldLocation _array_element) (* (Math|Rotator|GetRotationXVector (Transformation|GetWorldRotation _array_element)) (Math|Float|MakeLiteralFloat (Variables|Options|GetBeam%20lenght)))) "TraceTypeQuery1" true 0 "None"))
    (if _returnvalue
      ;;[1 1 1] If hit, set the end point to the hit location
      (Variables|Default|SetBeam%20end%20point (.ImpactPoint (Collision|BreakHitResult _outhit)))
      (else
        (Variables|Default|SetBeam%20end%20point (+ (Transformation|GetWorldLocation _array_element) (* (Math|Rotator|GetRotationXVector (Transformation|GetWorldRotation _array_element)) (Math|Float|MakeLiteralFloat (Variables|Options|GetBeam%20lenght)))))))
    ;;[1 1 1] Use this function to create the beam according to the defined start and end location
    (CallFunction|CreateBeam (Transformation|GetWorldLocation _array_element) (Variables|Default|GetBeam%20end%20point) false)))

(fn ConstructionScript)

(fn CreateBeam
  (params (Start :type Vector) (End :type Vector) (Destroy%20? :type Boolean))
  ;[1 1 1] Use this function to get the particle system corresponding to the selected color
  (bind _out (CallFunction|GetColor (Variables|Options|GetColor)))
  ;[1 1 1] Create the particle
  (bind _returnvalue (Effects|SpawnEmitteratLocation _out Start "0, 0, 0" "1.000000,1.000000,1.000000" Destroy%20?))
  (bind _output_get (Variables|Default|SetEmietter _returnvalue))
  (Class|ParticleSystemComponent|SetBeamEndPoint _output_get 0 End))

(fn GetColor
  (params (Color :type Colors%20Enum :default "NewEnumerator0"))
  ;[1 1 1] Depending on the selected color, output the corresponding laser particle system
  (switch Utilities|FlowControl|Switch|SwitchonColors Color
    (:NewEnumerator0
      (return "/Game/LaserPack/Particles/Laser_Blue.Laser_Blue"))
    (:NewEnumerator1
      (return "/Game/LaserPack/Particles/Laser_LightBlue.Laser_LightBlue"))
    (:NewEnumerator2
      (return "/Game/LaserPack/Particles/Laser_Purple.Laser_Purple"))
    (:NewEnumerator3
      (return "/Game/LaserPack/Particles/Laser_Red.Laser_Red"))
    (:NewEnumerator4
      (return "/Game/LaserPack/Particles/Laser_Pink.Laser_Pink"))
    (:NewEnumerator5
      (return "/Game/LaserPack/Particles/Laser_Orange.Laser_Orange"))
    (:NewEnumerator6
      (return "/Game/LaserPack/Particles/Laser_Yellow.Laser_Yellow"))
    (:NewEnumerator7
      (return "/Game/LaserPack/Particles/Laser_Green.Laser_Green"))
    (:NewEnumerator8
      (return "/Game/LaserPack/Particles/Laser_White.Laser_White"))
    (:NewEnumerator9
      (return "/Game/LaserPack/Particles/Laser_Off.Laser_Off"))))