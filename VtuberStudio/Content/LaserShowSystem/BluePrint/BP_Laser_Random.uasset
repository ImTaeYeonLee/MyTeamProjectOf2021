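; Laser show fixture that fires randomly scattered particle beams, with adjustable count, color or random hue, flicker and speed.
; Construction gathers "Target" bones; each beam update randomizes their positions on a hidden PoseableMesh and draws beams from the Center socket to them.
; Optional line traces cut beams at hit surfaces, and surplus beams get zero alpha.
; Tick also drives on/off and shutter strobing, and restarts a pitch-sweep timeline every half second.
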(event Custom|Laser02
  (bind _새_트랙_0 (Timeline|타임라인_1 PlayFromStart)))

(event Custom|Laser01
  (bind _returnvalue (Transformation|GetActorRotation))
  (bind _새_트랙_0 (Timeline|타임라인_0 PlayFromStart)
    (:Update
      (Transformation|SetActorRotation (Math|Rotator|MakeRotator (.roll _returnvalue) (- (.pitch _returnvalue) _새_트랙_0) (.yaw _returnvalue))))))

(event EventBeginPlay
  (bind _returnvalue (Actor|GetActorOfClass "/Game/TY/Maps/BP_Sound.BP_Sound_C"))
  (Variables|Default|SetBPSound _returnvalue))

(event EventTick
  (params (DeltaSeconds :type Float%20%28single-precision%29))
  (bind _beamarray (Variables|BeamSettings|GetBeamArray))
  (bind _number_max24_ (Variables|BeamSettings|GetNumber%28Max24%29))
  (bind _returnvalue (+ _number_max24_ 24))
  (Utilities|FlowControl|Sequence
    (:then_0
      ;[0 1 0.3804 0.498] Device ON/OFF
      (CallFunction|DeviceON/OFF)
      ;[0.1313 0.05115 1 0.5] Set Scale
      (Transformation|SetRelativeScale3D (Variables|Default|GetTriangle_with_bone) (* (Variables|GeneralSettings|GetScale) 5.0))
      ;[1 0 0 0.5] Shutter
      (|Shutter
        (:OutputPin
          ;[1 0.02331 0.8814 0.5] Set Speed
          (Utilities|FlowControl|Delay (* (Variables|BeamSettings|GetSpeed) 0.01))
          ;[0 1 0.7 0.5] Set Beams
          (for _index (range 24 _returnvalue)
            (CallFunction|Beam (Utilities|Array|Get(acopy) _beamarray _index) _index))
          ;;[0 1 0.6311 0.5] Hidden Beam set Alpha=0
          (for _index_2 (range _returnvalue 47)
            (Effects|Components|ParticleSystem|SetFloatParameter (Utilities|Array|Get(acopy) _beamarray _index_2) "Alpha" 0.0)))))
    (:then_1
      (Variables|Default|SetCurrentTime (+ DeltaSeconds (Variables|Default|GetCurrentTime)))
      (if (>= (Variables|Default|GetCurrentTime) 0.5)
        (CallFunction|Laser01)
        (CallFunction|Laser02)
        (Variables|Default|SetCurrentTime 0.0)))))

(fn ConstructionScript
  ;[0.9926 0.04479 1 0.5] Get all bone name and make array
  (|Bonenamearray
    (:NewParam
      ;[0 0.5 1 0.5] Set Beam array
      (Variables|BeamSettings|SetBeamArray (|MakeParticleSystemArray))
      ;[0 1 0.3804 0.498] Device ON/OFF
      (CallFunction|DeviceON/OFF)
      ;[0.1313 0.05115 1 0.5] Set Scale
      (Transformation|SetRelativeScale3D (Variables|Default|GetTriangle_with_bone) (* (Variables|GeneralSettings|GetScale) 5.0))
      (Utilities|FlowControl|Sequence
        (:then_0
          ;[1 0.3893 0 0.5] Set Surface
          (CallFunction|Fog))
        (:then_1
          ;[1 0 0.4201 0.5] Copy Bone(for target randomize)
          (Class|PoseableMeshComponent|CopyPosefromSkeletalComponent (Variables|Default|GetPoseableMesh) (Variables|Default|GetTriangle_with_bone)))
        (:then_2
          ;[0 1 0.7146 0.5] Set Beams
          (for _index (range 24 47)
            (CallFunction|Beam (Utilities|Array|Get(acopy) (Variables|BeamSettings|GetBeamArray) _index) _index)))))))

(fn Beam
  (params (ParticleSystem :type Particle%20System%20Component%20Object%20Reference) (TargetPoint :type Integer))
  (bind _returnvalue (Math|Random|RandomUnitVector))
  (bind _beam_color (Variables|BeamSettings|GetBeam%20Color))
  (bind _beam_thickness (Variables|BeamSettings|GetBeam%20Thickness))
  ;[0 1 0.4878 0.5] Beam Settings
  (Effects|Components|ParticleSystem|SetVectorParameter ParticleSystem "Scale" (Math|Vector|MakeVector _beam_thickness _beam_thickness _beam_thickness))
  (Effects|Components|ParticleSystem|SetColorParameter ParticleSystem "Color Over Life" (select (Variables|BeamSettings|GetHue%20Random) (Math|Conversions|ToLinearColor(Vector) (Math|Vector|SelectVector _returnvalue "1.000000,1.000000,1.000000" (Math|Vector|NotEqual(Vector) _returnvalue "0, 0, 0" 0.0001))) _beam_color))
  (Effects|Components|ParticleSystem|SetFloatParameter ParticleSystem "Alpha" (- (.A (Math|Color|BreakColor _beam_color)) (Math|Random|RandomFloatinRange 0.0 (/ (Variables|BeamSettings|GetFricker%20Beam) 1e+02))))
  ;[0 0.1811 1 0.5] Set Bone Random
  (Class|PoseableMeshComponent|SetBoneLocationbyName (Variables|Default|GetPoseableMesh) (Utilities|Array|Get(acopy) (Variables|BeamSettings|GetTargetNameArray) TargetPoint) (Math|Vector|MakeVector 1.5e+02 (Math|Random|RandomFloatinRange (Variables|BeamSettings|GetRandom%20Y%20Mini) (Variables|BeamSettings|GetRandom%20Y%20Max)) (Math|Random|RandomFloatinRange (Variables|BeamSettings|GetRandom%20X%20Mini) (Variables|BeamSettings|GetRandom%20X%20Max))) "ComponentSpace")
  ;[0.6831 0.01406 1 0.5] Set Beam Start / End point
  (Variables|BeamSettings|SetStartPoint (Transformation|GetSocketLocation (Variables|Default|GetTriangle_with_bone) "Center"))
  (Variables|BeamSettings|SetTargetPoint (Transformation|GetSocketLocation (Variables|Default|GetPoseableMesh) (Utilities|Array|Get(acopy) (Variables|BeamSettings|GetTargetNameArray) TargetPoint)))
  (Class|ParticleSystemComponent|SetBeamSourcePoint ParticleSystem 0 (Variables|BeamSettings|GetStartPoint))
  (if (Variables|BeamSettings|GetCut%20Off)
    ;[1 0.3647 0.01654 0.5] Get collision
    (bind _outhit (Collision|LineTraceByChannel (Variables|BeamSettings|GetStartPoint) (Variables|BeamSettings|GetTargetPoint) "TraceTypeQuery1" true 0 "None" true "(R=0.704039,G=0.000000,B=1.000000,A=1.000000)" "(R=1.000000,G=1.000000,B=0.000000,A=1.000000)" 0.5))
    (if (.bBlockingHit (Collision|BreakHitResult _outhit))
      ;;[1 0 0 0.5] Remove 0, 0, 0
      (if (Math|Vector|NotEqual(Vector) (.ImpactPoint (Collision|BreakHitResult _outhit)) "0, 0, 0" 0.0001)
        (Class|ParticleSystemComponent|SetBeamTargetPoint ParticleSystem 0 (.ImpactPoint (Collision|BreakHitResult _outhit))))
      (else
        (Class|ParticleSystemComponent|SetBeamTargetPoint ParticleSystem 0 (.TraceEnd (Collision|BreakHitResult _outhit)))))
    (else
      (Class|ParticleSystemComponent|SetBeamTargetPoint ParticleSystem 0 (Variables|BeamSettings|GetTargetPoint)))))

(fn Fog
  (Rendering|SetVisibility (Variables|Default|GetTriangle_with_bone) false false))

(fn DeviceON/OFF
  (bind _defaultsceneroot (Variables|Default|GetDefaultSceneRoot))
  (if (not (Variables|GeneralSettings|GetDevice%20OFF))
    (Rendering|SetVisibility _defaultsceneroot true true)
    (else
      (Rendering|SetVisibility _defaultsceneroot false true))))