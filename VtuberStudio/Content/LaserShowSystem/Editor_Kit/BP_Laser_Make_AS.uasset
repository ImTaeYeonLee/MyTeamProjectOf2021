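; Laser show actor that renders an animated fog surface on a boned triangle mesh with 48 particle beams.
; Construction gathers "Target" bone names, the beam array and a dynamic surface material.
; Construction and Tick run Update, which applies scale, fog parameters and beam settings with random alpha flicker.
; Beams run from the Center socket to target bones, optionally cut by line traces; a timeline shutter strobes visibility, alongside a device on/off switch.
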(event EventTick
  (params (DeltaSeconds :type Float%20%28single-precision%29))
  ;[0 1 0.3804 0.498] Device ON/OFF
  (CallFunction|DeviceON/OFF)
  ;[1 0 0 0.5] Shutter
  (|Shutter
    (:OutputPin
      ;[1 0.8333 0 0.3] Main function
      (CallFunction|Update))))

(fn ConstructionScript
  ;[0.9926 0.04479 1 0.5] Get all bone name and make array
  (|Bonenamearray
    (:NewParam
      ;[0 0.5 1 0.5] Set Beam array
      (Variables|BeamSettings|SetBeamArray (|MakeParticleSystemArray))
      ;[0 1 0.3804 0.498] Device ON/OFF
      (CallFunction|DeviceON/OFF)
      ;[1 0.2616 0 0.3] Set Dynamic Material Instance
      (bind _returnvalue (Rendering|Material|CreateDynamicMaterialInstance (Variables|Default|GetTriangle_with_bone) 0 "/Game/LaserShowSystem/Material/MI_Laser_Surface.MI_Laser_Surface" "None" :!class /Script/Engine.PrimitiveComponent))
      (Variables|Default|SetDynamicMaterialInstance _returnvalue)
      ;[1 0.8333 0 0.3] Main function
      (CallFunction|Update))))

(fn Beam
  (params (ParticleSystem :type Particle%20System%20Component%20Object%20Reference) (TargetPoint :type Integer))
  (bind _beam_color (Variables|BeamSettings|GetBeam%20Color))
  (bind _beam_thickness (Variables|BeamSettings|GetBeam%20Thickness))
  ;[0 1 0.4878 0.5] Beam Settings
  (Effects|Components|ParticleSystem|SetVectorParameter ParticleSystem "Scale" (Math|Vector|MakeVector _beam_thickness _beam_thickness _beam_thickness))
  (Effects|Components|ParticleSystem|SetColorParameter ParticleSystem "Color Over Life" _beam_color)
  (Effects|Components|ParticleSystem|SetFloatParameter ParticleSystem "Alpha" (- (.A (Math|Color|BreakColor _beam_color)) (Math|Random|RandomFloatinRange 0.0 (/ (Variables|BeamSettings|GetFricker%20Beam) 1e+02))))
  ;[0.6831 0.01406 1 0.5] Set Beam Start / End point
  (Variables|BeamSettings|SetStartPoint (Transformation|GetSocketLocation (Variables|Default|GetTriangle_with_bone) "Center"))
  (Variables|BeamSettings|SetTargetPoint (Transformation|GetSocketLocation (Variables|Default|GetTriangle_with_bone) (Utilities|Array|Get(acopy) (Variables|BeamSettings|GetTargetNameArray) TargetPoint)))
  (Class|ParticleSystemComponent|SetBeamSourcePoint ParticleSystem 0 (Variables|BeamSettings|GetStartPoint))
  (if (Variables|BeamSettings|GetCut%20Off)
    ;[1 0.3647 0.01654 0.5] Get collision
    (bind _outhit (Collision|LineTraceByChannel (Variables|BeamSettings|GetStartPoint) (Variables|BeamSettings|GetTargetPoint) "TraceTypeQuery1" true 0 "None" true "(R=0.704039,G=0.000000,B=1.000000,A=1.000000)" "(R=1.000000,G=1.000000,B=0.000000,A=1.000000)" 0.5))
    (if (.bBlockingHit (Collision|BreakHitResult _outhit))
      ;;[1 0 0 0.5] Remove 0, 0, 0
      (if (Math|Vector|NotEqual(Vector) (.ImpactPoint (Collision|BreakHitResult _outhit)) "0, 0, 0" 0.0001)
        (Class|ParticleSystemComponent|SetBeamTargetPoint ParticleSystem 0 (.ImpactPoint (Collision|BreakHitResult _outhit))))
      (else
        (Class|ParticleSystemComponent|SetBeamTargetPoint ParticleSystem 0 (.TraceEnd (Collision|BreakHitResult _outhit)))))
    (else
      (Class|ParticleSystemComponent|SetBeamTargetPoint ParticleSystem 0 (Variables|BeamSettings|GetTargetPoint)))))

(fn Surface
  (bind _dynamicmaterialinstance (Variables|Default|GetDynamicMaterialInstance))
  (bind _surface_color (Variables|FogGeneralSettings|GetSurface%20Color))
  ;[0.5 0 1 0.5] Fog General Settings
  (Rendering|Material|SetVectorParameterValue _dynamicmaterialinstance "Color" _surface_color :!class /Script/Engine.MaterialInstanceDynamic)
  (if (Variables|FogGeneralSettings|GetFog%20ON/OFF)
    (Rendering|Material|SetScalarParameterValue _dynamicmaterialinstance "Opacity" (- (.A (Math|Color|BreakColor _surface_color)) (Math|Random|RandomFloatinRange 0.0 (/ (Variables|FogGeneralSettings|GetFricker%20Fog) 1e+02))) :!class /Script/Engine.MaterialInstanceDynamic)
    (Rendering|Material|SetScalarParameterValue _dynamicmaterialinstance "Falloff" (Variables|FogGeneralSettings|GetFalloff) :!class /Script/Engine.MaterialInstanceDynamic)
    (Rendering|Material|SetScalarParameterValue _dynamicmaterialinstance "Emissive" (Variables|FogGeneralSettings|GetFog%20Emissive) :!class /Script/Engine.MaterialInstanceDynamic)
    (Rendering|Material|SetScalarParameterValue _dynamicmaterialinstance "Mix" (Variables|FogGeneralSettings|GetMix%28A/B%29) :!class /Script/Engine.MaterialInstanceDynamic)
    (Rendering|Material|SetScalarParameterValue _dynamicmaterialinstance "Edge Thickness" (Variables|FogGeneralSettings|GetEdge%20Thickness) :!class /Script/Engine.MaterialInstanceDynamic)
    (Rendering|Material|SetScalarParameterValue _dynamicmaterialinstance "Fog A Divide X" (Variables|FogASettings|GetFog%20A%20Divide%20X) :!class /Script/Engine.MaterialInstanceDynamic)
    (Rendering|Material|SetScalarParameterValue _dynamicmaterialinstance "Fog A Divide Y" (Variables|FogASettings|GetFog%20A%20Divide%20Y) :!class /Script/Engine.MaterialInstanceDynamic)
    (Rendering|Material|SetScalarParameterValue _dynamicmaterialinstance "Fog A Speed X" (* (Variables|FogASettings|GetFog%20A%20Speed%20X) (Variables|FogGeneralSettings|GetFog%20Speed)) :!class /Script/Engine.MaterialInstanceDynamic)
    (Rendering|Material|SetScalarParameterValue _dynamicmaterialinstance "Fog A Speed Y" (* (Variables|FogASettings|GetFog%20A%20Speed%20Y) (Variables|FogGeneralSettings|GetFog%20Speed)) :!class /Script/Engine.MaterialInstanceDynamic)
    (Rendering|Material|SetTextureParameterValue _dynamicmaterialinstance "Fog A Texture" (Variables|FogASettings|GetFog%20A%20Texture))
    ;[0 1 1 0.5] Fog B
    (Rendering|Material|SetScalarParameterValue _dynamicmaterialinstance "Fog B Divide X" (Variables|FogBSettings|GetFog%20B%20Divide%20X) :!class /Script/Engine.MaterialInstanceDynamic)
    (Rendering|Material|SetScalarParameterValue _dynamicmaterialinstance "Fog B Divide Y" (Variables|FogBSettings|GetFog%20B%20Divide%20Y) :!class /Script/Engine.MaterialInstanceDynamic)
    (Rendering|Material|SetScalarParameterValue _dynamicmaterialinstance "Fog B Speed X" (* (Variables|FogBSettings|GetFog%20B%20Speed%20X) (Variables|FogGeneralSettings|GetFog%20Speed)) :!class /Script/Engine.MaterialInstanceDynamic)
    (Rendering|Material|SetScalarParameterValue _dynamicmaterialinstance "Fog B Speed Y" (* (Variables|FogBSettings|GetFog%20B%20Speed%20Y) (Variables|FogGeneralSettings|GetFog%20Speed)) :!class /Script/Engine.MaterialInstanceDynamic)
    (Rendering|Material|SetTextureParameterValue _dynamicmaterialinstance "Fog B Texture" (Variables|FogBSettings|GetFog%20B%20Texture))
    (else
      (Rendering|Material|SetScalarParameterValue _dynamicmaterialinstance "Opacity" 0.0 :!class /Script/Engine.MaterialInstanceDynamic))))

(fn DeviceON/OFF
  (bind _defaultsceneroot (Variables|Default|GetDefaultSceneRoot))
  (if (not (Variables|GeneralSettings|GetDevice%20OFF))
    (Rendering|SetVisibility _defaultsceneroot true true)
    (else
      (Rendering|SetVisibility _defaultsceneroot false true))))

(fn Update
  ;[0.1313 0.05115 1 0.5] Set Scale
  (Transformation|SetRelativeScale3D (Variables|Default|GetTriangle_with_bone) (* (Variables|GeneralSettings|GetScale) 5.0))
  (Utilities|FlowControl|Sequence
    (:then_0
      ;[1 0.3893 0 0.5] Set Surface
      (CallFunction|Surface))
    (:then_1
      ;[0 1 0.7146 0.5] Set Beams
      (for _index (range 0 47)
        (CallFunction|Beam (Utilities|Array|Get(acopy) (Variables|BeamSettings|GetBeamArray) _index) _index)))))