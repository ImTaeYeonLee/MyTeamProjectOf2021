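; BP_MediaVisualizer is a placeable actor that plays a media source alongside an optional Niagara system, controlled by a box trigger.
; BeginPlay, if Sound is set, activates MediaSound and starts playback; box entry runs the same start chain without that activation.
; Starting reopens the source and resets and shows Niagara; exiting pauses, deactivates sound and hides Niagara.
; The construction script sizes the box and labels it with the source name.
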(event OnComponentBeginOverlap(Box)
  (params (OverlappedComponent :type Primitive%20Component%20Object%20Reference) (OtherActor :type Actor%20Object%20Reference) (OtherComp :type Primitive%20Component%20Object%20Reference) (OtherBodyIndex :type Integer) (bFromSweep :type Boolean) (SweepResult :type Hit%20Result%20Structure%20%28by%20ref%29))
  (bind _mediaplayer (Variables|Default|GetMediaPlayer))
  (Media|MediaPlayer|OpenSource _mediaplayer (Variables|Default|GetMedia%20Source))
  (Media|MediaSoundComponent|SetMediaPlayer (Variables|Default|GetMediaSound) _mediaplayer)
  (Media|MediaPlayer|Play _mediaplayer :!class /Script/MediaAssets.MediaPlayer)
  (Components|Timeline|SetLooping _mediaplayer (Variables|Default|GetLooping))
  (EventDispatchers|AssignOnEndReached _mediaplayer (delegate Custom|OnEndReached_Event_0))
  (bind _niagarasystem (Variables|Default|GetNiagaraSystem)
    (:then
      (Niagara|ReinitializeSystem (Variables|/Script/Niagara.NiagaraActor|GetNiagaraComponent _niagarasystem))
      (Niagara|ResetSystem (Variables|/Script/Niagara.NiagaraActor|GetNiagaraComponent _niagarasystem))
      (Rendering|SetVisibility (Variables|/Script/Niagara.NiagaraActor|GetNiagaraComponent _niagarasystem) true false))
    (:else)))

(event OnComponentEndOverlap(Box)
  (params (OverlappedComponent :type Primitive%20Component%20Object%20Reference) (OtherActor :type Actor%20Object%20Reference) (OtherComp :type Primitive%20Component%20Object%20Reference) (OtherBodyIndex :type Integer))
  (Sequencer|Player|Pause (Variables|Default|GetMediaPlayer))
  (Components|Activation|Deactivate (Variables|Default|GetMediaSound))
  (bind _niagarasystem (Variables|Default|GetNiagaraSystem)
    (:then
      (Components|Activation|Deactivate (Variables|/Script/Niagara.NiagaraActor|GetNiagaraComponent _niagarasystem))
      (Rendering|SetVisibility (Variables|/Script/Niagara.NiagaraActor|GetNiagaraComponent _niagarasystem) false false))
    (:else)))

(event Custom|OnEndReached_Event_0)

(event EventBeginPlay
  (bind _mediaplayer (Variables|Default|GetMediaPlayer))
  (Utilities|FlowControl|Sequence
    (:then_0
      (if (Variables|Default|GetSound)
        (Components|Activation|Activate (Variables|Default|GetMediaSound) false)
        (Media|MediaPlayer|OpenSource _mediaplayer (Variables|Default|GetMedia%20Source))
        (Media|MediaSoundComponent|SetMediaPlayer (Variables|Default|GetMediaSound) _mediaplayer)
        (Media|MediaPlayer|Play _mediaplayer :!class /Script/MediaAssets.MediaPlayer)
        (Components|Timeline|SetLooping _mediaplayer (Variables|Default|GetLooping))
        (EventDispatchers|AssignOnEndReached _mediaplayer (delegate Custom|OnEndReached_Event_0))
        (bind _niagarasystem (Variables|Default|GetNiagaraSystem)
          (:then
            (Niagara|ReinitializeSystem (Variables|/Script/Niagara.NiagaraActor|GetNiagaraComponent _niagarasystem))
            (Niagara|ResetSystem (Variables|/Script/Niagara.NiagaraActor|GetNiagaraComponent _niagarasystem))
            (Rendering|SetVisibility (Variables|/Script/Niagara.NiagaraActor|GetNiagaraComponent _niagarasystem) true false))
          (:else))))))

(event Collision|EventActorBeginOverlap
  (params (OtherActor :type Actor%20Object%20Reference)))

(event EventTick
  (params (DeltaSeconds :type Float%20%28single-precision%29)))

(fn ConstructionScript
  (bind _textrender (Variables|Default|GetTextRender))
  (Components|Box|SetBoxExtent (Variables|Default|GetBox) (Variables|Default|GetIn%20Box%20Extent) true)
  (Rendering|Components|TextRender|SetText _textrender (Utilities|Text|ToText(String) (Utilities|GetDisplayName (Variables|Default|GetMedia%20Source))))
  (Development|SetHiddeninGame _textrender (Variables|Default|GetText%20Hidden) false))