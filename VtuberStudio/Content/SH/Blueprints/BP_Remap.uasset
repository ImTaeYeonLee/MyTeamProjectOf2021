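; BP_Remap is a bone-name remap, likely for Live Link retargeting, translating mannequin-style bone names to VRM-style J_Bip names.
; GetRemappedBoneName switches on the incoming name and returns a hardcoded target for root, spine, neck, head, arms and legs, with no finger or toe entries.
; As written, Clavicle R returns the left shoulder, Root returns "Skelton", and Head L and Head R return the hand bones.
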(fn GetRemappedBoneName
  (params (BoneName :type Name :default "None"))
  (switch name BoneName
    (:Root
      (return "Skelton"))
    (:Pelvis
      (return "J_Bip_C_Hips"))
    (:spine_01
      (return "J_Bip_C_Spine"))
    (:spine_02
      (return "J_Bip_C_Chest"))
    (:spine_03
      (return "J_Bip_C_UpperChest"))
    (:clavicle_l
      (return "J_Bip_L_Shoulder"))
    (:UpperArm_L
      (return "J_Bip_L_UpperArm"))
    (:lowerarm_l
      (return "J_Bip_L_LowerArm"))
    (:Head_L
      (return "J_Bip_L_Hand"))
    (:clavicle_r
      (return "J_Bip_L_Shoulder"))
    (:UpperArm_R
      (return "J_Bip_R_UpperArm"))
    (:lowerarm_r
      (return "J_Bip_R_LowerArm"))
    (:Head_R
      (return "J_Bip_R_Hand"))
    (:neck_01
      (return "J_Bip_C_Neck"))
    (:head
      (return "J_Bip_C_Head"))
    (:Thigh_L
      (return "J_Bip_L_UpperLeg"))
    (:calf_i
      (return "J_Bip_L_LowerLeg"))
    (:Foot_L
      (return "J_Bip_L_Foot"))
    (:Thigh_R
      (return "J_Bip_R_UpperLeg"))
    (:calf_r
      (return "J_Bip_R_LowerLeg"))
    (:Foot_R
      (return "J_Bip_R_Foot"))))