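; SH_InfoImporter applies VRM import settings saved in the game instance when play begins.
; It reads the file name and import type from SH_BP_GameInstance and uses the ImportType map to turn that type into a VRM material type.
; It writes the material type into the first BP_dropActor's import options, then has that actor load the VRM from the saved path.
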(event EventBeginPlay
  ;[1 1 1] Instance에서 정보 가져오기
  (bind _outactors (Actor|GetAllActorsOfClass "/VRM4U/Util/Actor/Misc/BP_dropActor.BP_dropActor_C"))
  (bind _assh_bp_game_instance (Utilities|Casting|CastToSH_BP_GameInstance (Game|GetGameInstance)))
  (Variables|Default|SetAs%20SH%20BP%20Game%20Instance _assh_bp_game_instance)
  (Utilities|Struct|SetmembersinImportOptionData (Variables|/VRM4U/Util/Actor/Misc/BP_dropActor.BP_dropActor_C|GetImportOption (Utilities|Array|Get(acopy) _outactors)) (Utilities|Enum|ByteToEnumEVRMImportMaterialType (.Value (Utilities|Map|Find (Variables|Default|GetImportType) (Variables|/Game/SH/Blueprints/SH_BP_GameInstance.SH_BP_GameInstance_C|GetSH_ImportType (Variables|Default|GetAs%20SH%20BP%20Game%20Instance))))))
  (Default|LoadVrmFronFilePath (Utilities|Array|Get(acopy) _outactors) (Variables|/Game/SH/Blueprints/SH_BP_GameInstance.SH_BP_GameInstance_C|GetSH_VrmFileName (Variables|Default|GetAs%20SH%20BP%20Game%20Instance))))

(fn ConstructionScript)