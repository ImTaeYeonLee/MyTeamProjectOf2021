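; Helper Blueprint that makes VRM avatars loaded through BP_dropActor copy animation from a reference skeletal mesh, AnimRefTarget.
; On BeginPlay it finds the drop actor and binds to OnApplyNewVRM, then feeds the new asset list and reference mesh into the spawned avatar's VrmAnimInstanceCopy.
; An invalid reference mesh re-runs the lookup and binding.
; An unconnected looping graph alternates Fun and Blink blend shapes, resetting to neutral.
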(event Custom|CustomEvent_0
  (params (VRMAssetList :type Vrm%20Asset%20List%20Object%20Object%20Reference))
  (bind _animreftarget (Variables|Default|GetAnimRefTarget))
  (bind _skeletalmesh (Variables|/Game/SH/Blueprints/SH_BP_TrackingPawn.SH_BP_TrackingPawn_C|GetSkeletalMesh _animreftarget))
  ;[1 1 1] 애니메이션 레퍼런스 블루프린트 설정
  (bind _asvrm_anim_instance_copy (Utilities|Casting|CastToVrmAnimInstanceCopy (Components|SkeletalMesh|GetAnimInstance (Variables|/VRM4U/Util/Actor/MToonActor.MToonActor_C|GetSkeletalMesh (Variables|/VRM4U/Util/Actor/Misc/BP_dropActor.BP_dropActor_C|GetSpawnedActor (stale _returnvalue))))))
  ;;[1 1 1] VRM Ref 모델 정보 받아오기 예외처리
  (Utilities|IsValid _skeletalmesh
    (:Is%20Valid
      ;[1 1 1] set animation
      (Class|VrmAnimInstanceCopy|SetSkeletalMeshCopyData _asvrm_anim_instance_copy VRMAssetList _skeletalmesh "/VRM4U/Util/BaseCharacter/Mesh/VRoidSimple_VrmAssetList.VRoidSimple_VrmAssetList"))
    (:Is%20Not%20Valid
      (bind _returnvalue (Actor|GetActorOfClass "/VRM4U/Util/Actor/Misc/BP_dropActor.BP_dropActor_C"))
      (Variables|Default|SetDropActor _returnvalue)
      (EventDispatchers|AssignOnApplyNewVRM _returnvalue (delegate Custom|CustomEvent_0)))))

(event EventTick
  (params (DeltaSeconds :type Float%20%28single-precision%29))
  ;[1 1 1] morph target
)

(event EventBeginPlay
  ;[1 1 1] 애니메이션 레퍼런스 블루프린트 설정
  (bind _returnvalue (Actor|GetActorOfClass "/VRM4U/Util/Actor/Misc/BP_dropActor.BP_dropActor_C"))
  (Variables|Default|SetDropActor _returnvalue)
  (EventDispatchers|AssignOnApplyNewVRM _returnvalue (delegate Custom|CustomEvent_0)))

(fn ConstructionScript)