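; BP_Light_V2 is a configurable spotlight prop that pairs a cannon-light mesh with a SpotLight component.
; The construction script applies exposed-style variables for intensity, color, attenuation radius and inner and outer cone angles to the SpotLight.
; It also adds LightRotation to the mesh's current relative roll while zeroing pitch and yaw.
; The event graph holds only disabled stubs, so the Blueprint has no runtime logic.
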(event EventBeginPlay)

(event Collision|EventActorBeginOverlap
  (params (OtherActor :type Actor%20Object%20Reference)))

(event EventTick
  (params (DeltaSeconds :type Float%20%28single-precision%29)))

(fn ConstructionScript
  (bind _sm_cannonlight_v1 (Variables|Default|GetSM_CannonLight_V1))
  (bind _spotlight (Variables|Default|GetSpotLight))
  (Transformation|SetRelativeRotation _sm_cannonlight_v1 (Math|Rotator|MakeRotator (+ (.roll (Variables|/Script/Engine.SceneComponent|GetRelativeRotation _sm_cannonlight_v1)) (Variables|Default|GetLightRotation)) 0.0 0.0) false false)
  (Rendering|Components|Light|SetIntensity _spotlight (Variables|Default|GetLightIntensity))
  (Rendering|Components|Light|SetLightColor _spotlight (Variables|Default|GetLightColor) true)
  (Rendering|Lighting|SetAttenuationRadius _spotlight (Variables|Default|GetLightDistance))
  (Rendering|Lighting|SetInnerConeAngle _spotlight (Variables|Default|GetLightInnerCone))
  (Rendering|Lighting|SetOuterConeAngle _spotlight (Variables|Default|GetLightOuterCone)))