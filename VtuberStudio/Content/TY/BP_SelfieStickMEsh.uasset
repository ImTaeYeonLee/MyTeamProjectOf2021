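; Selfie stick actor made of a hand mesh and a stick mesh that can be attached and released.
; Released turns on custom depth with a stencil value on both meshes, for stencil-based effects, and Attached clears it.
; PhysicsOn enables physics simulation on both meshes and gravity on the hand.
; PhysicOff is empty, and the physics-off and stick-follows-hand nodes are left unconnected.
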(event Custom|Attached
  (bind _handmesh (Variables|Default|GetHandMesh))
  (bind _stickmesh (Variables|Default|GetStickMesh))
  ;[1 1 1] 잡았따!
  ;[1 1 1] 끄기
  (Rendering|SetRenderCustomDepth _handmesh false)
  (Rendering|SetCustomDepthStencilValue _handmesh 0)
  (Rendering|SetRenderCustomDepth _stickmesh false)
  (Rendering|SetCustomDepthStencilValue _stickmesh 0))

(event Custom|Released
  (bind _handmesh (Variables|Default|GetHandMesh))
  (bind _stickmesh (Variables|Default|GetStickMesh))
  ;[1 1 1] 놨따!
  ;[1 1 1] 켜기
  (Rendering|SetRenderCustomDepth _handmesh true)
  (Rendering|SetCustomDepthStencilValue _handmesh 2)
  (Rendering|SetRenderCustomDepth _stickmesh true)
  (Rendering|SetCustomDepthStencilValue _stickmesh 2))

(event Custom|PhysicOff)

(event Custom|PhysicsOn
  (Physics|SetSimulatePhysics (Variables|Default|GetHandMesh) true)
  (Physics|SetEnableGravity (Variables|Default|GetHandMesh) true))

(event EventBeginPlay)

(event Collision|EventActorBeginOverlap
  (params (OtherActor :type Actor%20Object%20Reference)))

(event EventTick
  (params (DeltaSeconds :type Float%20%28single-precision%29)))

(fn ConstructionScript)