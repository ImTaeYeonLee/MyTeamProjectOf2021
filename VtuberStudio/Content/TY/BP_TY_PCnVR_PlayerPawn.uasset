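; Player pawn for switching between PC and VR play, starting in VR mode with the HMD enabled.
; Tab toggles the HMD and the VRMod flag, while ChangeState applies the current flag to the HMD.
; Tick prints debug values for boost state, boost time and the PlayerMove speed; no movement or boost logic lives in these graphs.
; HMD status printouts and a VOIP talker node are left unwired and never run.
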(event EventBeginPlay
  (Class|HeadMountedDisplayFunctionLibrary|EnableHMD true)
  (if true
    (Variables|Default|SetVRMod true)
    (else
      (Variables|Default|SetVRMod false))))

(event Collision|EventActorBeginOverlap
  (params (OtherActor :type Actor%20Object%20Reference)))

(event EventTick
  (params (DeltaSeconds :type Float%20%28single-precision%29))
  (Development|PrintString (Utilities|String|ToString(Boolean) (Variables|Default|GetisBoost)))
  (Development|PrintString (Utilities|String|ToString(Float) (Variables|/Script/UE_VtuberStudio.TY_PC_MoveActorComponent|GetmoveSpeed (Variables|Default|GetplayerMove))))
  (Development|PrintString (Utilities|String|ToString(Float) (Variables|Default|GetboostTime))))

(event Input|KeyboardEvents|Tab
  (params (Key :type Key%20Structure :default "None"))
  ;[1 1 1] Tab 누르면 HMD 켜고 끄기
  (:Pressed
    (if (Variables|Default|GetVRMod)
      (Class|HeadMountedDisplayFunctionLibrary|EnableHMD false)
      (Variables|Default|SetVRMod false)
      (else
        (Class|HeadMountedDisplayFunctionLibrary|EnableHMD true)
        (Variables|Default|SetVRMod true)))))

(fn ConstructionScript)

(fn ChangeState
  (Class|HeadMountedDisplayFunctionLibrary|EnableHMD (Variables|Default|GetVRMod)))