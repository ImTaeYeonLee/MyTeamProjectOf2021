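; VR pickup actor for the selfie stick that relays its grab state to a BP_SelfieStickMesh actor to toggle the outline.
; BeginPlay caches the first BP_SelfieStickMesh in the level via GetActorOfClass.
; Tick polls IsAttaching and calls Attached or Released on the mesh every frame, and the actor's own Attached and Released events forward the same calls.
; The mesh's physics toggle calls are left unconnected.
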(event Custom|Attached
  (bind _asbp_selfie_stick_mesh (Utilities|Casting|CastToBP_SelfieStickMesh (Variables|Default|GetChildActor_StickMesh_Ref)))
  (Default|Attached _asbp_selfie_stick_mesh))

(event Custom|Released
  (bind _asbp_selfie_stick_mesh (Utilities|Casting|CastToBP_SelfieStickMesh (Variables|Default|GetChildActor_StickMesh_Ref)))
  (Default|Released _asbp_selfie_stick_mesh))

(event EventBeginPlay
  ;[1 1 1] 대상 캐싱
  (bind _returnvalue (Actor|GetActorOfClass "/Game/TY/BP_SelfieStickMEsh.BP_SelfieStickMesh_C"))
  (bind _output_get (Variables|Default|SetChildActor_StickMesh_Ref _returnvalue)))

(event Collision|EventActorBeginOverlap
  (params (OtherActor :type Actor%20Object%20Reference)))

(event EventTick
  (params (DeltaSeconds :type Float%20%28single-precision%29))
  ;[1 1 1] 테두리 켜고 끄기
  (if (Variables|Default|GetisAttaching)
    (Default|Attached (stale EventBeginPlay _output_get))
    (else
      (Default|Released (stale EventBeginPlay _output_get)))))

(fn ConstructionScript)