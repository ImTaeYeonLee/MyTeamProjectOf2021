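; BP_Sound plays a music track after a short delay and launches a timed Niagara firework show at hard-coded positions.
; Playback percent becomes PlayTime; three DoOnce-gated upper-bound time checks, all true at playback start, trigger the burst chain.
; Delay-chained spawns sweep inward, back outward, then fire volleys and zigzags.
; Holding H pauses audio via Tick; later willow and line-effect cues are disconnected.
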(event Custom|BurstEffect
  (bind _niagarablue (Variables|Default|GetNiagaraBlue))
  ;[1 1 1] Burst 끝부터
  (Niagara|SpawnSystematLocation "/Game/TY/NI_Burst_System_ColorSetting_Blue.NI_Burst_System_ColorSetting_Blue" "-800.000000,-260.000000,120.000000" "0, 0, 0" "0.200000,0.200000,0.200000")
  (Niagara|SpawnSystematLocation "/Game/TY/NI_Burst_System_ColorSetting_Blue.NI_Burst_System_ColorSetting_Blue" "800.000000,-260.000000,120.000000" "0, 0, 0" "0.200000,0.200000,0.200000")
  (Utilities|FlowControl|Delay 0.2)
  (Niagara|SpawnSystematLocation "/Game/TY/Effects/Niagara/NI_Burst_System.NI_Burst_System" "-680.000000,-430.000000,175.000000" "0, 0, 0" "0.200000,0.200000,0.200000")
  (Niagara|SpawnSystematLocation "/Game/TY/Effects/Niagara/NI_Burst_System.NI_Burst_System" "690.000000,-430.000000,175.000000" "0, 0, 0" "0.200000,0.200000,0.200000")
  (Utilities|FlowControl|Delay 0.2)
  (Niagara|SpawnSystematLocation "/Game/TY/Effects/Niagara/NI_Burst_System.NI_Burst_System" "-580.000000,-540.000000,175.000000" "0, 0, 0" "0.200000,0.200000,0.200000")
  (Niagara|SpawnSystematLocation "/Game/TY/Effects/Niagara/NI_Burst_System.NI_Burst_System" "590.000000,-540.000000,175.000000" "0, 0, 0" "0.200000,0.200000,0.200000")
  (Utilities|FlowControl|Delay 0.2)
  (Niagara|SpawnSystematLocation "/Game/TY/Effects/Niagara/NI_Burst_System.NI_Burst_System" "-470.000000,-650.000000,175.000000" "0, 0, 0" "0.200000,0.200000,0.200000")
  (Niagara|SpawnSystematLocation "/Game/TY/Effects/Niagara/NI_Burst_System.NI_Burst_System" "470.000000,-650.000000,175.000000" "0, 0, 0" "0.200000,0.200000,0.200000")
  (Utilities|FlowControl|Delay 0.5)
  ;[0 1 0.1083] Burst01 차례대로 1회
  (Utilities|FlowControl|Sequence
    (:then_0
      (Niagara|SpawnSystematLocation _niagarablue "0.000000,-680.000000,175.000000" "0, 0, 0" "0.200000,0.200000,0.200000")
      (Utilities|FlowControl|Delay 0.35)
      (Utilities|FlowControl|Sequence
        (:then_0
          (Niagara|SpawnSystematLocation _niagarablue "-580.000000,-540.000000,175.000000" "0, 0, 0" "0.200000,0.200000,0.200000")
          (Utilities|FlowControl|Delay 0.35)
          (Utilities|FlowControl|Sequence
            (:then_0
              (Niagara|SpawnSystematLocation _niagarablue "-680.000000,-430.000000,175.000000" "0, 0, 0" "0.200000,0.200000,0.200000")
              (Utilities|FlowControl|Delay 0.35)
              (Utilities|FlowControl|Sequence
                (:then_0
                  (Niagara|SpawnSystematLocation "/Game/TY/Effects/Niagara/NI_Burst_System.NI_Burst_System" "-800.000000,-260.000000,120.000000" "0, 0, 0" "0.200000,0.200000,0.200000")
                  (Utilities|FlowControl|Delay 0.5)
                  ;[0 1 0.1083] Burst02 다같이 3회
                  (Utilities|FlowControl|Sequence
                    (:then_0
                      (Niagara|SpawnSystematLocation "/Game/TY/Effects/Niagara/NI_Burst_System.NI_Burst_System" "0.000000,-680.000000,175.000000" "0, 0, 0" "0.200000,0.200000,0.200000")
                      (Utilities|FlowControl|Delay 0.6)
                      (Utilities|FlowControl|Sequence
                        (:then_0
                          (Niagara|SpawnSystematLocation "/Game/TY/Effects/Niagara/NI_Burst_System.NI_Burst_System" "0.000000,-680.000000,175.000000" "0, 0, 0" "0.200000,0.200000,0.200000")
                          (Utilities|FlowControl|Delay 0.6)
                          (Utilities|FlowControl|Sequence
                            (:then_0
                              (Niagara|SpawnSystematLocation "/Game/TY/Effects/Niagara/NI_Burst_System.NI_Burst_System" "0.000000,-680.000000,175.000000" "0, 0, 0" "0.200000,0.200000,0.200000")
                              (Utilities|FlowControl|Delay 0.5)
                              ;[0 1 0.1798] 지그재그 1회
                              (Niagara|SpawnSystematLocation "/Game/TY/Effects/Niagara/NI_Burst_System.NI_Burst_System" "0.000000,-680.000000,175.000000" "0, 0, 0" "0.200000,0.200000,0.200000")
                              (Niagara|SpawnSystematLocation "/Game/TY/Effects/Niagara/NI_Burst_System.NI_Burst_System" "-580.000000,-540.000000,175.000000" "0, 0, 0" "0.200000,0.200000,0.200000")
                              (Niagara|SpawnSystematLocation "/Game/TY/Effects/Niagara/NI_Burst_System.NI_Burst_System" "590.000000,-540.000000,175.000000" "0, 0, 0" "0.200000,0.200000,0.200000")
                              (Niagara|SpawnSystematLocation "/Game/TY/Effects/Niagara/NI_Burst_System.NI_Burst_System" "-800.000000,-260.000000,120.000000" "0, 0, 0" "0.200000,0.200000,0.200000")
                              (Niagara|SpawnSystematLocation "/Game/TY/Effects/Niagara/NI_Burst_System.NI_Burst_System" "800.000000,-260.000000,120.000000" "0, 0, 0" "0.200000,0.200000,0.200000")
                              (Utilities|FlowControl|Delay 1.0)
                              (Niagara|SpawnSystematLocation "/Game/TY/Effects/Niagara/NI_Burst_System.NI_Burst_System" "-680.000000,-430.000000,175.000000" "0, 0, 0" "0.200000,0.200000,0.200000")
                              (Niagara|SpawnSystematLocation "/Game/TY/Effects/Niagara/NI_Burst_System.NI_Burst_System" "690.000000,-430.000000,175.000000" "0, 0, 0" "0.200000,0.200000,0.200000")
                              (Niagara|SpawnSystematLocation "/Game/TY/Effects/Niagara/NI_Burst_System.NI_Burst_System" "-470.000000,-650.000000,175.000000" "0, 0, 0" "0.200000,0.200000,0.200000")
                              (Niagara|SpawnSystematLocation "/Game/TY/Effects/Niagara/NI_Burst_System.NI_Burst_System" "470.000000,-650.000000,175.000000" "0, 0, 0" "0.200000,0.200000,0.200000")
                              (Niagara|SpawnSystematLocation "/Game/TY/Effects/Niagara/NI_Burst_System.NI_Burst_System" "0.000000,-680.000000,175.000000" "0, 0, 0" "0.200000,0.200000,0.200000")
                              (Utilities|FlowControl|Delay 1.2)
                              ;[0 1 0.1798] 지그재그 1회
                              (Niagara|SpawnSystematLocation "/Game/TY/Effects/Niagara/NI_Burst_System.NI_Burst_System" "0.000000,-680.000000,175.000000" "0, 0, 0" "0.200000,0.200000,0.200000")
                              (Niagara|SpawnSystematLocation "/Game/TY/Effects/Niagara/NI_Burst_System.NI_Burst_System" "-580.000000,-540.000000,175.000000" "0, 0, 0" "0.200000,0.200000,0.200000")
                              (Niagara|SpawnSystematLocation "/Game/TY/Effects/Niagara/NI_Burst_System.NI_Burst_System" "590.000000,-540.000000,175.000000" "0, 0, 0" "0.200000,0.200000,0.200000")
                              (Niagara|SpawnSystematLocation "/Game/TY/Effects/Niagara/NI_Burst_System.NI_Burst_System" "-800.000000,-260.000000,120.000000" "0, 0, 0" "0.200000,0.200000,0.200000")
                              (Niagara|SpawnSystematLocation "/Game/TY/Effects/Niagara/NI_Burst_System.NI_Burst_System" "800.000000,-260.000000,120.000000" "0, 0, 0" "0.200000,0.200000,0.200000")
                              (Utilities|FlowControl|Delay 1.0)
                              (Niagara|SpawnSystematLocation "/Game/TY/Effects/Niagara/NI_Burst_System.NI_Burst_System" "-680.000000,-430.000000,175.000000" "0, 0, 0" "0.200000,0.200000,0.200000")
                              (Niagara|SpawnSystematLocation "/Game/TY/Effects/Niagara/NI_Burst_System.NI_Burst_System" "690.000000,-430.000000,175.000000" "0, 0, 0" "0.200000,0.200000,0.200000")
                              (Niagara|SpawnSystematLocation "/Game/TY/Effects/Niagara/NI_Burst_System.NI_Burst_System" "-470.000000,-650.000000,175.000000" "0, 0, 0" "0.200000,0.200000,0.200000")
                              (Niagara|SpawnSystematLocation "/Game/TY/Effects/Niagara/NI_Burst_System.NI_Burst_System" "470.000000,-650.000000,175.000000" "0, 0, 0" "0.200000,0.200000,0.200000")
                              (Niagara|SpawnSystematLocation "/Game/TY/Effects/Niagara/NI_Burst_System.NI_Burst_System" "0.000000,-680.000000,175.000000" "0, 0, 0" "0.200000,0.200000,0.200000")
                              (Utilities|FlowControl|Delay 1.2)
                              ;[0 1 0.1798] 지그재그 1회
                              (Niagara|SpawnSystematLocation "/Game/TY/Effects/Niagara/NI_Burst_System.NI_Burst_System" "0.000000,-680.000000,175.000000" "0, 0, 0" "0.200000,0.200000,0.200000")
                              (Niagara|SpawnSystematLocation "/Game/TY/Effects/Niagara/NI_Burst_System.NI_Burst_System" "-580.000000,-540.000000,175.000000" "0, 0, 0" "0.200000,0.200000,0.200000")
                              (Niagara|SpawnSystematLocation "/Game/TY/Effects/Niagara/NI_Burst_System.NI_Burst_System" "590.000000,-540.000000,175.000000" "0, 0, 0" "0.200000,0.200000,0.200000")
                              (Niagara|SpawnSystematLocation "/Game/TY/Effects/Niagara/NI_Burst_System.NI_Burst_System" "-800.000000,-260.000000,120.000000" "0, 0, 0" "0.200000,0.200000,0.200000")
                              (Niagara|SpawnSystematLocation "/Game/TY/Effects/Niagara/NI_Burst_System.NI_Burst_System" "800.000000,-260.000000,120.000000" "0, 0, 0" "0.200000,0.200000,0.200000")
                              (Utilities|FlowControl|Delay 1.0)
                              (Niagara|SpawnSystematLocation "/Game/TY/Effects/Niagara/NI_Burst_System.NI_Burst_System" "-680.000000,-430.000000,175.000000" "0, 0, 0" "0.200000,0.200000,0.200000")
                              (Niagara|SpawnSystematLocation "/Game/TY/Effects/Niagara/NI_Burst_System.NI_Burst_System" "690.000000,-430.000000,175.000000" "0, 0, 0" "0.200000,0.200000,0.200000")
                              (Niagara|SpawnSystematLocation "/Game/TY/Effects/Niagara/NI_Burst_System.NI_Burst_System" "-470.000000,-650.000000,175.000000" "0, 0, 0" "0.200000,0.200000,0.200000")
                              (Niagara|SpawnSystematLocation "/Game/TY/Effects/Niagara/NI_Burst_System.NI_Burst_System" "470.000000,-650.000000,175.000000" "0, 0, 0" "0.200000,0.200000,0.200000")
                              (Niagara|SpawnSystematLocation "/Game/TY/Effects/Niagara/NI_Burst_System.NI_Burst_System" "0.000000,-680.000000,175.000000" "0, 0, 0" "0.200000,0.200000,0.200000"))
                            (:then_1
                              (Niagara|SpawnSystematLocation "/Game/TY/Effects/Niagara/NI_Burst_System.NI_Burst_System" "-470.000000,-650.000000,175.000000" "0, 0, 0" "0.200000,0.200000,0.200000"))
                            (:then_2
                              (Niagara|SpawnSystematLocation "/Game/TY/Effects/Niagara/NI_Burst_System.NI_Burst_System" "470.000000,-650.000000,175.000000" "0, 0, 0" "0.200000,0.200000,0.200000"))
                            (:then_3
                              (Niagara|SpawnSystematLocation "/Game/TY/Effects/Niagara/NI_Burst_System.NI_Burst_System" "-580.000000,-540.000000,175.000000" "0, 0, 0" "0.200000,0.200000,0.200000"))
                            (:then_4
                              (Niagara|SpawnSystematLocation "/Game/TY/Effects/Niagara/NI_Burst_System.NI_Burst_System" "590.000000,-540.000000,175.000000" "0, 0, 0" "0.200000,0.200000,0.200000"))
                            (:then_5
                              (Niagara|SpawnSystematLocation "/Game/TY/Effects/Niagara/NI_Burst_System.NI_Burst_System" "-680.000000,-430.000000,175.000000" "0, 0, 0" "0.200000,0.200000,0.200000"))
                            (:then_6
                              (Niagara|SpawnSystematLocation "/Game/TY/Effects/Niagara/NI_Burst_System.NI_Burst_System" "690.000000,-430.000000,175.000000" "0, 0, 0" "0.200000,0.200000,0.200000"))
                            (:then_7
                              (Niagara|SpawnSystematLocation "/Game/TY/Effects/Niagara/NI_Burst_System.NI_Burst_System" "-800.000000,-260.000000,120.000000" "0, 0, 0" "0.200000,0.200000,0.200000"))
                            (:then_8
                              (Niagara|SpawnSystematLocation "/Game/TY/Effects/Niagara/NI_Burst_System.NI_Burst_System" "800.000000,-260.000000,120.000000" "0, 0, 0" "0.200000,0.200000,0.200000"))))
                        (:then_1
                          (Niagara|SpawnSystematLocation "/Game/TY/Effects/Niagara/NI_Burst_System.NI_Burst_System" "-470.000000,-650.000000,175.000000" "0, 0, 0" "0.200000,0.200000,0.200000"))
                        (:then_2
                          (Niagara|SpawnSystematLocation "/Game/TY/Effects/Niagara/NI_Burst_System.NI_Burst_System" "470.000000,-650.000000,175.000000" "0, 0, 0" "0.200000,0.200000,0.200000"))
                        (:then_3
                          (Niagara|SpawnSystematLocation "/Game/TY/Effects/Niagara/NI_Burst_System.NI_Burst_System" "-580.000000,-540.000000,175.000000" "0, 0, 0" "0.200000,0.200000,0.200000"))
                        (:then_4
                          (Niagara|SpawnSystematLocation "/Game/TY/Effects/Niagara/NI_Burst_System.NI_Burst_System" "590.000000,-540.000000,175.000000" "0, 0, 0" "0.200000,0.200000,0.200000"))
                        (:then_5
                          (Niagara|SpawnSystematLocation "/Game/TY/Effects/Niagara/NI_Burst_System.NI_Burst_System" "-680.000000,-430.000000,175.000000" "0, 0, 0" "0.200000,0.200000,0.200000"))
                        (:then_6
                          (Niagara|SpawnSystematLocation "/Game/TY/Effects/Niagara/NI_Burst_System.NI_Burst_System" "690.000000,-430.000000,175.000000" "0, 0, 0" "0.200000,0.200000,0.200000"))
                        (:then_7
                          (Niagara|SpawnSystematLocation "/Game/TY/Effects/Niagara/NI_Burst_System.NI_Burst_System" "-800.000000,-260.000000,120.000000" "0, 0, 0" "0.200000,0.200000,0.200000"))
                        (:then_8
                          (Niagara|SpawnSystematLocation "/Game/TY/Effects/Niagara/NI_Burst_System.NI_Burst_System" "800.000000,-260.000000,120.000000" "0, 0, 0" "0.200000,0.200000,0.200000"))))
                    (:then_1
                      (Niagara|SpawnSystematLocation "/Game/TY/Effects/Niagara/NI_Burst_System.NI_Burst_System" "-470.000000,-650.000000,175.000000" "0, 0, 0" "0.200000,0.200000,0.200000"))
                    (:then_2
                      (Niagara|SpawnSystematLocation "/Game/TY/Effects/Niagara/NI_Burst_System.NI_Burst_System" "470.000000,-650.000000,175.000000" "0, 0, 0" "0.200000,0.200000,0.200000"))
                    (:then_3
                      (Niagara|SpawnSystematLocation "/Game/TY/Effects/Niagara/NI_Burst_System.NI_Burst_System" "-580.000000,-540.000000,175.000000" "0, 0, 0" "0.200000,0.200000,0.200000"))
                    (:then_4
                      (Niagara|SpawnSystematLocation "/Game/TY/Effects/Niagara/NI_Burst_System.NI_Burst_System" "590.000000,-540.000000,175.000000" "0, 0, 0" "0.200000,0.200000,0.200000"))
                    (:then_5
                      (Niagara|SpawnSystematLocation "/Game/TY/Effects/Niagara/NI_Burst_System.NI_Burst_System" "-680.000000,-430.000000,175.000000" "0, 0, 0" "0.200000,0.200000,0.200000"))
                    (:then_6
                      (Niagara|SpawnSystematLocation "/Game/TY/Effects/Niagara/NI_Burst_System.NI_Burst_System" "690.000000,-430.000000,175.000000" "0, 0, 0" "0.200000,0.200000,0.200000"))
                    (:then_7
                      (Niagara|SpawnSystematLocation "/Game/TY/Effects/Niagara/NI_Burst_System.NI_Burst_System" "-800.000000,-260.000000,120.000000" "0, 0, 0" "0.200000,0.200000,0.200000"))
                    (:then_8
                      (Niagara|SpawnSystematLocation "/Game/TY/Effects/Niagara/NI_Burst_System.NI_Burst_System" "800.000000,-260.000000,120.000000" "0, 0, 0" "0.200000,0.200000,0.200000"))))
                (:then_1
                  (Niagara|SpawnSystematLocation _niagarablue "800.000000,-260.000000,120.000000" "0, 0, 0" "0.200000,0.200000,0.200000"))))
            (:then_1
              (Niagara|SpawnSystematLocation _niagarablue "690.000000,-430.000000,175.000000" "0, 0, 0" "0.200000,0.200000,0.200000"))))
        (:then_1
          (Niagara|SpawnSystematLocation _niagarablue "590.000000,-540.000000,175.000000" "0, 0, 0" "0.200000,0.200000,0.200000"))))
    (:then_1
      (Niagara|SpawnSystematLocation _niagarablue "-470.000000,-650.000000,175.000000" "0, 0, 0" "0.200000,0.200000,0.200000"))
    (:then_2
      (Niagara|SpawnSystematLocation _niagarablue "470.000000,-650.000000,175.000000" "0, 0, 0" "0.200000,0.200000,0.200000"))))

(event Custom|PlaybackPercentEvent
  (params (PlayingSoundWave :type Sound%20Wave%20Object%20Reference) (PlaybackPercent :type Float%20%28single-precision%29))
  (bind _niagarablue (Variables|Default|GetNiagaraBlue))
  ;[1 1 1] 재생시간 받아오기
  (bind _output_get (Variables|Default|SetPlayTime (* PlaybackPercent (Variables|Default|GetSoundDuration))))
  (Development|PrintString (Utilities|String|ToString(Float) _output_get))
  (Utilities|FlowControl|Sequence
    (:then_0
      (if (>= 17.0 _output_get)
        (Utilities|FlowControl|DoOnce false
          (:Completed
            ;[1 1 1] Burst 끝부터
            (Niagara|SpawnSystematLocation "/Game/TY/NI_Burst_System_ColorSetting_Blue.NI_Burst_System_ColorSetting_Blue" "-800.000000,-260.000000,120.000000" "0, 0, 0" "0.200000,0.200000,0.200000" :!label _label)
            (Niagara|SpawnSystematLocation "/Game/TY/NI_Burst_System_ColorSetting_Blue.NI_Burst_System_ColorSetting_Blue" "800.000000,-260.000000,120.000000" "0, 0, 0" "0.200000,0.200000,0.200000")
            (Utilities|FlowControl|Delay 0.2)
            (Niagara|SpawnSystematLocation "/Game/TY/Effects/Niagara/NI_Burst_System.NI_Burst_System" "-680.000000,-430.000000,175.000000" "0, 0, 0" "0.200000,0.200000,0.200000")
            (Niagara|SpawnSystematLocation "/Game/TY/Effects/Niagara/NI_Burst_System.NI_Burst_System" "690.000000,-430.000000,175.000000" "0, 0, 0" "0.200000,0.200000,0.200000")
            (Utilities|FlowControl|Delay 0.2)
            (Niagara|SpawnSystematLocation "/Game/TY/Effects/Niagara/NI_Burst_System.NI_Burst_System" "-580.000000,-540.000000,175.000000" "0, 0, 0" "0.200000,0.200000,0.200000")
            (Niagara|SpawnSystematLocation "/Game/TY/Effects/Niagara/NI_Burst_System.NI_Burst_System" "590.000000,-540.000000,175.000000" "0, 0, 0" "0.200000,0.200000,0.200000")
            (Utilities|FlowControl|Delay 0.2)
            (Niagara|SpawnSystematLocation "/Game/TY/Effects/Niagara/NI_Burst_System.NI_Burst_System" "-470.000000,-650.000000,175.000000" "0, 0, 0" "0.200000,0.200000,0.200000")
            (Niagara|SpawnSystematLocation "/Game/TY/Effects/Niagara/NI_Burst_System.NI_Burst_System" "470.000000,-650.000000,175.000000" "0, 0, 0" "0.200000,0.200000,0.200000")
            (Utilities|FlowControl|Delay 0.5)
            ;[0 1 0.1083] Burst01 차례대로 1회
            (Utilities|FlowControl|Sequence
              (:then_0
                (Niagara|SpawnSystematLocation _niagarablue "0.000000,-680.000000,175.000000" "0, 0, 0" "0.200000,0.200000,0.200000")
                (Utilities|FlowControl|Delay 0.35)
                (Utilities|FlowControl|Sequence
                  (:then_0
                    (Niagara|SpawnSystematLocation _niagarablue "-580.000000,-540.000000,175.000000" "0, 0, 0" "0.200000,0.200000,0.200000")
                    (Utilities|FlowControl|Delay 0.35)
                    (Utilities|FlowControl|Sequence
                      (:then_0
                        (Niagara|SpawnSystematLocation _niagarablue "-680.000000,-430.000000,175.000000" "0, 0, 0" "0.200000,0.200000,0.200000")
                        (Utilities|FlowControl|Delay 0.35)
                        (Utilities|FlowControl|Sequence
                          (:then_0
                            (Niagara|SpawnSystematLocation "/Game/TY/Effects/Niagara/NI_Burst_System.NI_Burst_System" "-800.000000,-260.000000,120.000000" "0, 0, 0" "0.200000,0.200000,0.200000")
                            (Utilities|FlowControl|Delay 0.5)
                            ;[0 1 0.1083] Burst02 다같이 3회
                            (Utilities|FlowControl|Sequence
                              (:then_0
                                (Niagara|SpawnSystematLocation "/Game/TY/Effects/Niagara/NI_Burst_System.NI_Burst_System" "0.000000,-680.000000,175.000000" "0, 0, 0" "0.200000,0.200000,0.200000")
                                (Utilities|FlowControl|Delay 0.6)
                                (Utilities|FlowControl|Sequence
                                  (:then_0
                                    (Niagara|SpawnSystematLocation "/Game/TY/Effects/Niagara/NI_Burst_System.NI_Burst_System" "0.000000,-680.000000,175.000000" "0, 0, 0" "0.200000,0.200000,0.200000")
                                    (Utilities|FlowControl|Delay 0.6)
                                    (Utilities|FlowControl|Sequence
                                      (:then_0
                                        (Niagara|SpawnSystematLocation "/Game/TY/Effects/Niagara/NI_Burst_System.NI_Burst_System" "0.000000,-680.000000,175.000000" "0, 0, 0" "0.200000,0.200000,0.200000")
                                        (Utilities|FlowControl|Delay 0.5)
                                        ;[0 1 0.1798] 지그재그 1회
                                        (Niagara|SpawnSystematLocation "/Game/TY/Effects/Niagara/NI_Burst_System.NI_Burst_System" "0.000000,-680.000000,175.000000" "0, 0, 0" "0.200000,0.200000,0.200000")
                                        (Niagara|SpawnSystematLocation "/Game/TY/Effects/Niagara/NI_Burst_System.NI_Burst_System" "-580.000000,-540.000000,175.000000" "0, 0, 0" "0.200000,0.200000,0.200000")
                                        (Niagara|SpawnSystematLocation "/Game/TY/Effects/Niagara/NI_Burst_System.NI_Burst_System" "590.000000,-540.000000,175.000000" "0, 0, 0" "0.200000,0.200000,0.200000")
                                        (Niagara|SpawnSystematLocation "/Game/TY/Effects/Niagara/NI_Burst_System.NI_Burst_System" "-800.000000,-260.000000,120.000000" "0, 0, 0" "0.200000,0.200000,0.200000")
                                        (Niagara|SpawnSystematLocation "/Game/TY/Effects/Niagara/NI_Burst_System.NI_Burst_System" "800.000000,-260.000000,120.000000" "0, 0, 0" "0.200000,0.200000,0.200000")
                                        (Utilities|FlowControl|Delay 1.0)
                                        (Niagara|SpawnSystematLocation "/Game/TY/Effects/Niagara/NI_Burst_System.NI_Burst_System" "-680.000000,-430.000000,175.000000" "0, 0, 0" "0.200000,0.200000,0.200000")
                                        (Niagara|SpawnSystematLocation "/Game/TY/Effects/Niagara/NI_Burst_System.NI_Burst_System" "690.000000,-430.000000,175.000000" "0, 0, 0" "0.200000,0.200000,0.200000")
                                        (Niagara|SpawnSystematLocation "/Game/TY/Effects/Niagara/NI_Burst_System.NI_Burst_System" "-470.000000,-650.000000,175.000000" "0, 0, 0" "0.200000,0.200000,0.200000")
                                        (Niagara|SpawnSystematLocation "/Game/TY/Effects/Niagara/NI_Burst_System.NI_Burst_System" "470.000000,-650.000000,175.000000" "0, 0, 0" "0.200000,0.200000,0.200000")
                                        (Niagara|SpawnSystematLocation "/Game/TY/Effects/Niagara/NI_Burst_System.NI_Burst_System" "0.000000,-680.000000,175.000000" "0, 0, 0" "0.200000,0.200000,0.200000")
                                        (Utilities|FlowControl|Delay 1.2)
                                        ;[0 1 0.1798] 지그재그 1회
                                        (Niagara|SpawnSystematLocation "/Game/TY/Effects/Niagara/NI_Burst_System.NI_Burst_System" "0.000000,-680.000000,175.000000" "0, 0, 0" "0.200000,0.200000,0.200000")
                                        (Niagara|SpawnSystematLocation "/Game/TY/Effects/Niagara/NI_Burst_System.NI_Burst_System" "-580.000000,-540.000000,175.000000" "0, 0, 0" "0.200000,0.200000,0.200000")
                                        (Niagara|SpawnSystematLocation "/Game/TY/Effects/Niagara/NI_Burst_System.NI_Burst_System" "590.000000,-540.000000,175.000000" "0, 0, 0" "0.200000,0.200000,0.200000")
                                        (Niagara|SpawnSystematLocation "/Game/TY/Effects/Niagara/NI_Burst_System.NI_Burst_System" "-800.000000,-260.000000,120.000000" "0, 0, 0" "0.200000,0.200000,0.200000")
                                        (Niagara|SpawnSystematLocation "/Game/TY/Effects/Niagara/NI_Burst_System.NI_Burst_System" "800.000000,-260.000000,120.000000" "0, 0, 0" "0.200000,0.200000,0.200000")
                                        (Utilities|FlowControl|Delay 1.0)
                                        (Niagara|SpawnSystematLocation "/Game/TY/Effects/Niagara/NI_Burst_System.NI_Burst_System" "-680.000000,-430.000000,175.000000" "0, 0, 0" "0.200000,0.200000,0.200000")
                                        (Niagara|SpawnSystematLocation "/Game/TY/Effects/Niagara/NI_Burst_System.NI_Burst_System" "690.000000,-430.000000,175.000000" "0, 0, 0" "0.200000,0.200000,0.200000")
                                        (Niagara|SpawnSystematLocation "/Game/TY/Effects/Niagara/NI_Burst_System.NI_Burst_System" "-470.000000,-650.000000,175.000000" "0, 0, 0" "0.200000,0.200000,0.200000")
                                        (Niagara|SpawnSystematLocation "/Game/TY/Effects/Niagara/NI_Burst_System.NI_Burst_System" "470.000000,-650.000000,175.000000" "0, 0, 0" "0.200000,0.200000,0.200000")
                                        (Niagara|SpawnSystematLocation "/Game/TY/Effects/Niagara/NI_Burst_System.NI_Burst_System" "0.000000,-680.000000,175.000000" "0, 0, 0" "0.200000,0.200000,0.200000")
                                        (Utilities|FlowControl|Delay 1.2)
                                        ;[0 1 0.1798] 지그재그 1회
                                        (Niagara|SpawnSystematLocation "/Game/TY/Effects/Niagara/NI_Burst_System.NI_Burst_System" "0.000000,-680.000000,175.000000" "0, 0, 0" "0.200000,0.200000,0.200000")
                                        (Niagara|SpawnSystematLocation "/Game/TY/Effects/Niagara/NI_Burst_System.NI_Burst_System" "-580.000000,-540.000000,175.000000" "0, 0, 0" "0.200000,0.200000,0.200000")
                                        (Niagara|SpawnSystematLocation "/Game/TY/Effects/Niagara/NI_Burst_System.NI_Burst_System" "590.000000,-540.000000,175.000000" "0, 0, 0" "0.200000,0.200000,0.200000")
                                        (Niagara|SpawnSystematLocation "/Game/TY/Effects/Niagara/NI_Burst_System.NI_Burst_System" "-800.000000,-260.000000,120.000000" "0, 0, 0" "0.200000,0.200000,0.200000")
                                        (Niagara|SpawnSystematLocation "/Game/TY/Effects/Niagara/NI_Burst_System.NI_Burst_System" "800.000000,-260.000000,120.000000" "0, 0, 0" "0.200000,0.200000,0.200000")
                                        (Utilities|FlowControl|Delay 1.0)
                                        (Niagara|SpawnSystematLocation "/Game/TY/Effects/Niagara/NI_Burst_System.NI_Burst_System" "-680.000000,-430.000000,175.000000" "0, 0, 0" "0.200000,0.200000,0.200000")
                                        (Niagara|SpawnSystematLocation "/Game/TY/Effects/Niagara/NI_Burst_System.NI_Burst_System" "690.000000,-430.000000,175.000000" "0, 0, 0" "0.200000,0.200000,0.200000")
                                        (Niagara|SpawnSystematLocation "/Game/TY/Effects/Niagara/NI_Burst_System.NI_Burst_System" "-470.000000,-650.000000,175.000000" "0, 0, 0" "0.200000,0.200000,0.200000")
                                        (Niagara|SpawnSystematLocation "/Game/TY/Effects/Niagara/NI_Burst_System.NI_Burst_System" "470.000000,-650.000000,175.000000" "0, 0, 0" "0.200000,0.200000,0.200000")
                                        (Niagara|SpawnSystematLocation "/Game/TY/Effects/Niagara/NI_Burst_System.NI_Burst_System" "0.000000,-680.000000,175.000000" "0, 0, 0" "0.200000,0.200000,0.200000"))
                                      (:then_1
                                        (Niagara|SpawnSystematLocation "/Game/TY/Effects/Niagara/NI_Burst_System.NI_Burst_System" "-470.000000,-650.000000,175.000000" "0, 0, 0" "0.200000,0.200000,0.200000"))
                                      (:then_2
                                        (Niagara|SpawnSystematLocation "/Game/TY/Effects/Niagara/NI_Burst_System.NI_Burst_System" "470.000000,-650.000000,175.000000" "0, 0, 0" "0.200000,0.200000,0.200000"))
                                      (:then_3
                                        (Niagara|SpawnSystematLocation "/Game/TY/Effects/Niagara/NI_Burst_System.NI_Burst_System" "-580.000000,-540.000000,175.000000" "0, 0, 0" "0.200000,0.200000,0.200000"))
                                      (:then_4
                                        (Niagara|SpawnSystematLocation "/Game/TY/Effects/Niagara/NI_Burst_System.NI_Burst_System" "590.000000,-540.000000,175.000000" "0, 0, 0" "0.200000,0.200000,0.200000"))
                                      (:then_5
                                        (Niagara|SpawnSystematLocation "/Game/TY/Effects/Niagara/NI_Burst_System.NI_Burst_System" "-680.000000,-430.000000,175.000000" "0, 0, 0" "0.200000,0.200000,0.200000"))
                                      (:then_6
                                        (Niagara|SpawnSystematLocation "/Game/TY/Effects/Niagara/NI_Burst_System.NI_Burst_System" "690.000000,-430.000000,175.000000" "0, 0, 0" "0.200000,0.200000,0.200000"))
                                      (:then_7
                                        (Niagara|SpawnSystematLocation "/Game/TY/Effects/Niagara/NI_Burst_System.NI_Burst_System" "-800.000000,-260.000000,120.000000" "0, 0, 0" "0.200000,0.200000,0.200000"))
                                      (:then_8
                                        (Niagara|SpawnSystematLocation "/Game/TY/Effects/Niagara/NI_Burst_System.NI_Burst_System" "800.000000,-260.000000,120.000000" "0, 0, 0" "0.200000,0.200000,0.200000"))))
                                  (:then_1
                                    (Niagara|SpawnSystematLocation "/Game/TY/Effects/Niagara/NI_Burst_System.NI_Burst_System" "-470.000000,-650.000000,175.000000" "0, 0, 0" "0.200000,0.200000,0.200000"))
                                  (:then_2
                                    (Niagara|SpawnSystematLocation "/Game/TY/Effects/Niagara/NI_Burst_System.NI_Burst_System" "470.000000,-650.000000,175.000000" "0, 0, 0" "0.200000,0.200000,0.200000"))
                                  (:then_3
                                    (Niagara|SpawnSystematLocation "/Game/TY/Effects/Niagara/NI_Burst_System.NI_Burst_System" "-580.000000,-540.000000,175.000000" "0, 0, 0" "0.200000,0.200000,0.200000"))
                                  (:then_4
                                    (Niagara|SpawnSystematLocation "/Game/TY/Effects/Niagara/NI_Burst_System.NI_Burst_System" "590.000000,-540.000000,175.000000" "0, 0, 0" "0.200000,0.200000,0.200000"))
                                  (:then_5
                                    (Niagara|SpawnSystematLocation "/Game/TY/Effects/Niagara/NI_Burst_System.NI_Burst_System" "-680.000000,-430.000000,175.000000" "0, 0, 0" "0.200000,0.200000,0.200000"))
                                  (:then_6
                                    (Niagara|SpawnSystematLocation "/Game/TY/Effects/Niagara/NI_Burst_System.NI_Burst_System" "690.000000,-430.000000,175.000000" "0, 0, 0" "0.200000,0.200000,0.200000"))
                                  (:then_7
                                    (Niagara|SpawnSystematLocation "/Game/TY/Effects/Niagara/NI_Burst_System.NI_Burst_System" "-800.000000,-260.000000,120.000000" "0, 0, 0" "0.200000,0.200000,0.200000"))
                                  (:then_8
                                    (Niagara|SpawnSystematLocation "/Game/TY/Effects/Niagara/NI_Burst_System.NI_Burst_System" "800.000000,-260.000000,120.000000" "0, 0, 0" "0.200000,0.200000,0.200000"))))
                              (:then_1
                                (Niagara|SpawnSystematLocation "/Game/TY/Effects/Niagara/NI_Burst_System.NI_Burst_System" "-470.000000,-650.000000,175.000000" "0, 0, 0" "0.200000,0.200000,0.200000"))
                              (:then_2
                                (Niagara|SpawnSystematLocation "/Game/TY/Effects/Niagara/NI_Burst_System.NI_Burst_System" "470.000000,-650.000000,175.000000" "0, 0, 0" "0.200000,0.200000,0.200000"))
                              (:then_3
                                (Niagara|SpawnSystematLocation "/Game/TY/Effects/Niagara/NI_Burst_System.NI_Burst_System" "-580.000000,-540.000000,175.000000" "0, 0, 0" "0.200000,0.200000,0.200000"))
                              (:then_4
                                (Niagara|SpawnSystematLocation "/Game/TY/Effects/Niagara/NI_Burst_System.NI_Burst_System" "590.000000,-540.000000,175.000000" "0, 0, 0" "0.200000,0.200000,0.200000"))
                              (:then_5
                                (Niagara|SpawnSystematLocation "/Game/TY/Effects/Niagara/NI_Burst_System.NI_Burst_System" "-680.000000,-430.000000,175.000000" "0, 0, 0" "0.200000,0.200000,0.200000"))
                              (:then_6
                                (Niagara|SpawnSystematLocation "/Game/TY/Effects/Niagara/NI_Burst_System.NI_Burst_System" "690.000000,-430.000000,175.000000" "0, 0, 0" "0.200000,0.200000,0.200000"))
                              (:then_7
                                (Niagara|SpawnSystematLocation "/Game/TY/Effects/Niagara/NI_Burst_System.NI_Burst_System" "-800.000000,-260.000000,120.000000" "0, 0, 0" "0.200000,0.200000,0.200000"))
                              (:then_8
                                (Niagara|SpawnSystematLocation "/Game/TY/Effects/Niagara/NI_Burst_System.NI_Burst_System" "800.000000,-260.000000,120.000000" "0, 0, 0" "0.200000,0.200000,0.200000"))))
                          (:then_1
                            (Niagara|SpawnSystematLocation _niagarablue "800.000000,-260.000000,120.000000" "0, 0, 0" "0.200000,0.200000,0.200000"))))
                      (:then_1
                        (Niagara|SpawnSystematLocation _niagarablue "690.000000,-430.000000,175.000000" "0, 0, 0" "0.200000,0.200000,0.200000"))))
                  (:then_1
                    (Niagara|SpawnSystematLocation _niagarablue "590.000000,-540.000000,175.000000" "0, 0, 0" "0.200000,0.200000,0.200000"))))
              (:then_1
                (Niagara|SpawnSystematLocation _niagarablue "-470.000000,-650.000000,175.000000" "0, 0, 0" "0.200000,0.200000,0.200000"))
              (:then_2
                (Niagara|SpawnSystematLocation _niagarablue "470.000000,-650.000000,175.000000" "0, 0, 0" "0.200000,0.200000,0.200000")))))))
    (:then_1
      (if (>= 2.0 _output_get)
        (Utilities|FlowControl|DoOnce false
          (:Completed
            (goto _label)))))
    (:then_2
      (if (>= 3e+01 _output_get)
        (Utilities|FlowControl|DoOnce false
          (:Completed
            (goto _label)))))))

(event Custom|FireBurst
  (bind _niagarablue (Variables|Default|GetNiagaraBlue))
  ;[0 1 0.1083] Burst01 차례대로 1회
  (Utilities|FlowControl|Sequence
    (:then_0
      (Niagara|SpawnSystematLocation _niagarablue "0.000000,-680.000000,175.000000" "0, 0, 0" "0.200000,0.200000,0.200000")
      (Utilities|FlowControl|Delay 0.35)
      (Utilities|FlowControl|Sequence
        (:then_0
          (Niagara|SpawnSystematLocation _niagarablue "-580.000000,-540.000000,175.000000" "0, 0, 0" "0.200000,0.200000,0.200000")
          (Utilities|FlowControl|Delay 0.35)
          (Utilities|FlowControl|Sequence
            (:then_0
              (Niagara|SpawnSystematLocation _niagarablue "-680.000000,-430.000000,175.000000" "0, 0, 0" "0.200000,0.200000,0.200000")
              (Utilities|FlowControl|Delay 0.35)
              (Utilities|FlowControl|Sequence
                (:then_0
                  (Niagara|SpawnSystematLocation "/Game/TY/Effects/Niagara/NI_Burst_System.NI_Burst_System" "-800.000000,-260.000000,120.000000" "0, 0, 0" "0.200000,0.200000,0.200000")
                  (Utilities|FlowControl|Delay 0.5)
                  ;[0 1 0.1083] Burst02 다같이 3회
                  (Utilities|FlowControl|Sequence
                    (:then_0
                      (Niagara|SpawnSystematLocation "/Game/TY/Effects/Niagara/NI_Burst_System.NI_Burst_System" "0.000000,-680.000000,175.000000" "0, 0, 0" "0.200000,0.200000,0.200000")
                      (Utilities|FlowControl|Delay 0.6)
                      (Utilities|FlowControl|Sequence
                        (:then_0
                          (Niagara|SpawnSystematLocation "/Game/TY/Effects/Niagara/NI_Burst_System.NI_Burst_System" "0.000000,-680.000000,175.000000" "0, 0, 0" "0.200000,0.200000,0.200000")
                          (Utilities|FlowControl|Delay 0.6)
                          (Utilities|FlowControl|Sequence
                            (:then_0
                              (Niagara|SpawnSystematLocation "/Game/TY/Effects/Niagara/NI_Burst_System.NI_Burst_System" "0.000000,-680.000000,175.000000" "0, 0, 0" "0.200000,0.200000,0.200000")
                              (Utilities|FlowControl|Delay 0.5)
                              ;[0 1 0.1798] 지그재그 1회
                              (Niagara|SpawnSystematLocation "/Game/TY/Effects/Niagara/NI_Burst_System.NI_Burst_System" "0.000000,-680.000000,175.000000" "0, 0, 0" "0.200000,0.200000,0.200000")
                              (Niagara|SpawnSystematLocation "/Game/TY/Effects/Niagara/NI_Burst_System.NI_Burst_System" "-580.000000,-540.000000,175.000000" "0, 0, 0" "0.200000,0.200000,0.200000")
                              (Niagara|SpawnSystematLocation "/Game/TY/Effects/Niagara/NI_Burst_System.NI_Burst_System" "590.000000,-540.000000,175.000000" "0, 0, 0" "0.200000,0.200000,0.200000")
                              (Niagara|SpawnSystematLocation "/Game/TY/Effects/Niagara/NI_Burst_System.NI_Burst_System" "-800.000000,-260.000000,120.000000" "0, 0, 0" "0.200000,0.200000,0.200000")
                              (Niagara|SpawnSystematLocation "/Game/TY/Effects/Niagara/NI_Burst_System.NI_Burst_System" "800.000000,-260.000000,120.000000" "0, 0, 0" "0.200000,0.200000,0.200000")
                              (Utilities|FlowControl|Delay 1.0)
                              (Niagara|SpawnSystematLocation "/Game/TY/Effects/Niagara/NI_Burst_System.NI_Burst_System" "-680.000000,-430.000000,175.000000" "0, 0, 0" "0.200000,0.200000,0.200000")
                              (Niagara|SpawnSystematLocation "/Game/TY/Effects/Niagara/NI_Burst_System.NI_Burst_System" "690.000000,-430.000000,175.000000" "0, 0, 0" "0.200000,0.200000,0.200000")
                              (Niagara|SpawnSystematLocation "/Game/TY/Effects/Niagara/NI_Burst_System.NI_Burst_System" "-470.000000,-650.000000,175.000000" "0, 0, 0" "0.200000,0.200000,0.200000")
                              (Niagara|SpawnSystematLocation "/Game/TY/Effects/Niagara/NI_Burst_System.NI_Burst_System" "470.000000,-650.000000,175.000000" "0, 0, 0" "0.200000,0.200000,0.200000")
                              (Niagara|SpawnSystematLocation "/Game/TY/Effects/Niagara/NI_Burst_System.NI_Burst_System" "0.000000,-680.000000,175.000000" "0, 0, 0" "0.200000,0.200000,0.200000")
                              (Utilities|FlowControl|Delay 1.2)
                              ;[0 1 0.1798] 지그재그 1회
                              (Niagara|SpawnSystematLocation "/Game/TY/Effects/Niagara/NI_Burst_System.NI_Burst_System" "0.000000,-680.000000,175.000000" "0, 0, 0" "0.200000,0.200000,0.200000")
                              (Niagara|SpawnSystematLocation "/Game/TY/Effects/Niagara/NI_Burst_System.NI_Burst_System" "-580.000000,-540.000000,175.000000" "0, 0, 0" "0.200000,0.200000,0.200000")
                              (Niagara|SpawnSystematLocation "/Game/TY/Effects/Niagara/NI_Burst_System.NI_Burst_System" "590.000000,-540.000000,175.000000" "0, 0, 0" "0.200000,0.200000,0.200000")
                              (Niagara|SpawnSystematLocation "/Game/TY/Effects/Niagara/NI_Burst_System.NI_Burst_System" "-800.000000,-260.000000,120.000000" "0, 0, 0" "0.200000,0.200000,0.200000")
                              (Niagara|SpawnSystematLocation "/Game/TY/Effects/Niagara/NI_Burst_System.NI_Burst_System" "800.000000,-260.000000,120.000000" "0, 0, 0" "0.200000,0.200000,0.200000")
                              (Utilities|FlowControl|Delay 1.0)
                              (Niagara|SpawnSystematLocation "/Game/TY/Effects/Niagara/NI_Burst_System.NI_Burst_System" "-680.000000,-430.000000,175.000000" "0, 0, 0" "0.200000,0.200000,0.200000")
                              (Niagara|SpawnSystematLocation "/Game/TY/Effects/Niagara/NI_Burst_System.NI_Burst_System" "690.000000,-430.000000,175.000000" "0, 0, 0" "0.200000,0.200000,0.200000")
                              (Niagara|SpawnSystematLocation "/Game/TY/Effects/Niagara/NI_Burst_System.NI_Burst_System" "-470.000000,-650.000000,175.000000" "0, 0, 0" "0.200000,0.200000,0.200000")
                              (Niagara|SpawnSystematLocation "/Game/TY/Effects/Niagara/NI_Burst_System.NI_Burst_System" "470.000000,-650.000000,175.000000" "0, 0, 0" "0.200000,0.200000,0.200000")
                              (Niagara|SpawnSystematLocation "/Game/TY/Effects/Niagara/NI_Burst_System.NI_Burst_System" "0.000000,-680.000000,175.000000" "0, 0, 0" "0.200000,0.200000,0.200000")
                              (Utilities|FlowControl|Delay 1.2)
                              ;[0 1 0.1798] 지그재그 1회
                              (Niagara|SpawnSystematLocation "/Game/TY/Effects/Niagara/NI_Burst_System.NI_Burst_System" "0.000000,-680.000000,175.000000" "0, 0, 0" "0.200000,0.200000,0.200000")
                              (Niagara|SpawnSystematLocation "/Game/TY/Effects/Niagara/NI_Burst_System.NI_Burst_System" "-580.000000,-540.000000,175.000000" "0, 0, 0" "0.200000,0.200000,0.200000")
                              (Niagara|SpawnSystematLocation "/Game/TY/Effects/Niagara/NI_Burst_System.NI_Burst_System" "590.000000,-540.000000,175.000000" "0, 0, 0" "0.200000,0.200000,0.200000")
                              (Niagara|SpawnSystematLocation "/Game/TY/Effects/Niagara/NI_Burst_System.NI_Burst_System" "-800.000000,-260.000000,120.000000" "0, 0, 0" "0.200000,0.200000,0.200000")
                              (Niagara|SpawnSystematLocation "/Game/TY/Effects/Niagara/NI_Burst_System.NI_Burst_System" "800.000000,-260.000000,120.000000" "0, 0, 0" "0.200000,0.200000,0.200000")
                              (Utilities|FlowControl|Delay 1.0)
                              (Niagara|SpawnSystematLocation "/Game/TY/Effects/Niagara/NI_Burst_System.NI_Burst_System" "-680.000000,-430.000000,175.000000" "0, 0, 0" "0.200000,0.200000,0.200000")
                              (Niagara|SpawnSystematLocation "/Game/TY/Effects/Niagara/NI_Burst_System.NI_Burst_System" "690.000000,-430.000000,175.000000" "0, 0, 0" "0.200000,0.200000,0.200000")
                              (Niagara|SpawnSystematLocation "/Game/TY/Effects/Niagara/NI_Burst_System.NI_Burst_System" "-470.000000,-650.000000,175.000000" "0, 0, 0" "0.200000,0.200000,0.200000")
                              (Niagara|SpawnSystematLocation "/Game/TY/Effects/Niagara/NI_Burst_System.NI_Burst_System" "470.000000,-650.000000,175.000000" "0, 0, 0" "0.200000,0.200000,0.200000")
                              (Niagara|SpawnSystematLocation "/Game/TY/Effects/Niagara/NI_Burst_System.NI_Burst_System" "0.000000,-680.000000,175.000000" "0, 0, 0" "0.200000,0.200000,0.200000"))
                            (:then_1
                              (Niagara|SpawnSystematLocation "/Game/TY/Effects/Niagara/NI_Burst_System.NI_Burst_System" "-470.000000,-650.000000,175.000000" "0, 0, 0" "0.200000,0.200000,0.200000"))
                            (:then_2
                              (Niagara|SpawnSystematLocation "/Game/TY/Effects/Niagara/NI_Burst_System.NI_Burst_System" "470.000000,-650.000000,175.000000" "0, 0, 0" "0.200000,0.200000,0.200000"))
                            (:then_3
                              (Niagara|SpawnSystematLocation "/Game/TY/Effects/Niagara/NI_Burst_System.NI_Burst_System" "-580.000000,-540.000000,175.000000" "0, 0, 0" "0.200000,0.200000,0.200000"))
                            (:then_4
                              (Niagara|SpawnSystematLocation "/Game/TY/Effects/Niagara/NI_Burst_System.NI_Burst_System" "590.000000,-540.000000,175.000000" "0, 0, 0" "0.200000,0.200000,0.200000"))
                            (:then_5
                              (Niagara|SpawnSystematLocation "/Game/TY/Effects/Niagara/NI_Burst_System.NI_Burst_System" "-680.000000,-430.000000,175.000000" "0, 0, 0" "0.200000,0.200000,0.200000"))
                            (:then_6
                              (Niagara|SpawnSystematLocation "/Game/TY/Effects/Niagara/NI_Burst_System.NI_Burst_System" "690.000000,-430.000000,175.000000" "0, 0, 0" "0.200000,0.200000,0.200000"))
                            (:then_7
                              (Niagara|SpawnSystematLocation "/Game/TY/Effects/Niagara/NI_Burst_System.NI_Burst_System" "-800.000000,-260.000000,120.000000" "0, 0, 0" "0.200000,0.200000,0.200000"))
                            (:then_8
                              (Niagara|SpawnSystematLocation "/Game/TY/Effects/Niagara/NI_Burst_System.NI_Burst_System" "800.000000,-260.000000,120.000000" "0, 0, 0" "0.200000,0.200000,0.200000"))))
                        (:then_1
                          (Niagara|SpawnSystematLocation "/Game/TY/Effects/Niagara/NI_Burst_System.NI_Burst_System" "-470.000000,-650.000000,175.000000" "0, 0, 0" "0.200000,0.200000,0.200000"))
                        (:then_2
                          (Niagara|SpawnSystematLocation "/Game/TY/Effects/Niagara/NI_Burst_System.NI_Burst_System" "470.000000,-650.000000,175.000000" "0, 0, 0" "0.200000,0.200000,0.200000"))
                        (:then_3
                          (Niagara|SpawnSystematLocation "/Game/TY/Effects/Niagara/NI_Burst_System.NI_Burst_System" "-580.000000,-540.000000,175.000000" "0, 0, 0" "0.200000,0.200000,0.200000"))
                        (:then_4
                          (Niagara|SpawnSystematLocation "/Game/TY/Effects/Niagara/NI_Burst_System.NI_Burst_System" "590.000000,-540.000000,175.000000" "0, 0, 0" "0.200000,0.200000,0.200000"))
                        (:then_5
                          (Niagara|SpawnSystematLocation "/Game/TY/Effects/Niagara/NI_Burst_System.NI_Burst_System" "-680.000000,-430.000000,175.000000" "0, 0, 0" "0.200000,0.200000,0.200000"))
                        (:then_6
                          (Niagara|SpawnSystematLocation "/Game/TY/Effects/Niagara/NI_Burst_System.NI_Burst_System" "690.000000,-430.000000,175.000000" "0, 0, 0" "0.200000,0.200000,0.200000"))
                        (:then_7
                          (Niagara|SpawnSystematLocation "/Game/TY/Effects/Niagara/NI_Burst_System.NI_Burst_System" "-800.000000,-260.000000,120.000000" "0, 0, 0" "0.200000,0.200000,0.200000"))
                        (:then_8
                          (Niagara|SpawnSystematLocation "/Game/TY/Effects/Niagara/NI_Burst_System.NI_Burst_System" "800.000000,-260.000000,120.000000" "0, 0, 0" "0.200000,0.200000,0.200000"))))
                    (:then_1
                      (Niagara|SpawnSystematLocation "/Game/TY/Effects/Niagara/NI_Burst_System.NI_Burst_System" "-470.000000,-650.000000,175.000000" "0, 0, 0" "0.200000,0.200000,0.200000"))
                    (:then_2
                      (Niagara|SpawnSystematLocation "/Game/TY/Effects/Niagara/NI_Burst_System.NI_Burst_System" "470.000000,-650.000000,175.000000" "0, 0, 0" "0.200000,0.200000,0.200000"))
                    (:then_3
                      (Niagara|SpawnSystematLocation "/Game/TY/Effects/Niagara/NI_Burst_System.NI_Burst_System" "-580.000000,-540.000000,175.000000" "0, 0, 0" "0.200000,0.200000,0.200000"))
                    (:then_4
                      (Niagara|SpawnSystematLocation "/Game/TY/Effects/Niagara/NI_Burst_System.NI_Burst_System" "590.000000,-540.000000,175.000000" "0, 0, 0" "0.200000,0.200000,0.200000"))
                    (:then_5
                      (Niagara|SpawnSystematLocation "/Game/TY/Effects/Niagara/NI_Burst_System.NI_Burst_System" "-680.000000,-430.000000,175.000000" "0, 0, 0" "0.200000,0.200000,0.200000"))
                    (:then_6
                      (Niagara|SpawnSystematLocation "/Game/TY/Effects/Niagara/NI_Burst_System.NI_Burst_System" "690.000000,-430.000000,175.000000" "0, 0, 0" "0.200000,0.200000,0.200000"))
                    (:then_7
                      (Niagara|SpawnSystematLocation "/Game/TY/Effects/Niagara/NI_Burst_System.NI_Burst_System" "-800.000000,-260.000000,120.000000" "0, 0, 0" "0.200000,0.200000,0.200000"))
                    (:then_8
                      (Niagara|SpawnSystematLocation "/Game/TY/Effects/Niagara/NI_Burst_System.NI_Burst_System" "800.000000,-260.000000,120.000000" "0, 0, 0" "0.200000,0.200000,0.200000"))))
                (:then_1
                  (Niagara|SpawnSystematLocation _niagarablue "800.000000,-260.000000,120.000000" "0, 0, 0" "0.200000,0.200000,0.200000"))))
            (:then_1
              (Niagara|SpawnSystematLocation _niagarablue "690.000000,-430.000000,175.000000" "0, 0, 0" "0.200000,0.200000,0.200000"))))
        (:then_1
          (Niagara|SpawnSystematLocation _niagarablue "590.000000,-540.000000,175.000000" "0, 0, 0" "0.200000,0.200000,0.200000"))))
    (:then_1
      (Niagara|SpawnSystematLocation _niagarablue "-470.000000,-650.000000,175.000000" "0, 0, 0" "0.200000,0.200000,0.200000"))
    (:then_2
      (Niagara|SpawnSystematLocation _niagarablue "470.000000,-650.000000,175.000000" "0, 0, 0" "0.200000,0.200000,0.200000"))))

(event EventBeginPlay
  ;[1 1 1] 재생시간 받아오기
  (Utilities|FlowControl|Delay 2.0)
  (Variables|Default|SetSoundDuration (Variables|/Script/Engine.SoundBase|GetDuration (Variables|Default|GetSoundWave)))
  (EventDispatchers|BindEventtoOnAudioPlaybackPercent (Variables|Default|GetAudio) (delegate Custom|PlaybackPercentEvent))
  (Audio|Components|Audio|SetSound (Variables|Default|GetAudio) (Variables|Default|GetSoundWave))
  (Audio|Components|Audio|Play (Variables|Default|GetAudio) 0.0)
  (Variables|Default|SetNiagaraBlue "/Game/TY/NI_Burst_System_ColorSetting_Blue.NI_Burst_System_ColorSetting_Blue"))

(event Collision|EventActorBeginOverlap
  (params (OtherActor :type Actor%20Object%20Reference)))

(event EventTick
  (params (DeltaSeconds :type Float%20%28single-precision%29))
  (bind _audiopause (Variables|Default|GetAudioPause))
  (bind _audio (Variables|Default|GetAudio))
  ;[1 1 1] 재생시간 받아오기
  (if _audiopause
    (Development|PrintString (Utilities|String|ToString(Boolean) _audiopause))
    (Class|AudioComponent|SetPaused _audio true)
    (else
      (Class|AudioComponent|SetPaused _audio false))))

(event Input|KeyboardEvents|H
  (params (Key :type Key%20Structure :default "None"))
  (:Pressed
    (Variables|Default|SetAudioPause true))
  (:Released
    (Variables|Default|SetAudioPause false)))

(fn ConstructionScript)