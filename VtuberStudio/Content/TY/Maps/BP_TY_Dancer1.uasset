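; BP_TY_Dancer1 is a dancer pawn that walks to its marked spot in the level after a timed delay.
; On BeginPlay it stores the first DancerLoc_01 actor found in the world as its target.
; Tick accumulates elapsed time and, once MoveTime is reached, issues AIMoveTo toward that target with a very tight acceptance radius.
; The timer never resets, so the move request repeats every frame from then on.
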(event EventBeginPlay
  ;[1 1 1] 월드에서 모든 클래스 찾아서
  (bind _outactors (Actor|GetAllActorsOfClass "/Game/TY/Maps/DancerLoc_01.DancerLoc_01_C"))
  ;[1 1 1] 사본 가져와서 정의
  (Variables|Default|SetDancer%20Loc%2001 (Utilities|Array|Get(acopy) _outactors)))

(event Collision|EventActorBeginOverlap
  (params (OtherActor :type Actor%20Object%20Reference)))

(event EventTick
  (params (DeltaSeconds :type Float%20%28single-precision%29))
  (Variables|Default|SetCurrentTime (+ DeltaSeconds (Variables|Default|GetCurrentTime)))
  (if (>= (Variables|Default|GetCurrentTime) (Variables|Default|GetMoveTime))
    (AI|AIMoveTo self "0, 0, 0" (Variables|Default|GetDancer%20Loc%2001) 0.1 false)))

(fn ConstructionScript)