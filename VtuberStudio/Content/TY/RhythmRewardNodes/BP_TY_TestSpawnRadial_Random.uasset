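; Test actor for spawning rhythm reward nodes that, as wired, only calls Spin every Tick.
; BeginPlay caches the SoundWave's duration and deactivates its audio component; the playback-percent handler only computes played time, and its binding is disconnected.
; Disconnected leftovers hold timed CircleShot calls and audio-analysis experiments: onset-triggered Spin, ConstantQ cube scaling, and gated spawning of BP_TY_RhythmRewardNode scaled by banded loudness multipliers.
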(event Custom|PlaybackPercentEvent
  (params (PlayingSoundWave :type Sound%20Wave%20Object%20Reference) (PlaybackPercent :type Float%20%28single-precision%29))
  (Variables|Default|SetPlayedTime (* PlaybackPercent (Variables|Default|GetSoundDuration)))
  (Utilities|FlowControl|Sequence))

(event Collision|EventActorBeginOverlap
  (params (OtherActor :type Actor%20Object%20Reference)))

(event EventTick
  (params (DeltaSeconds :type Float%20%28single-precision%29))
  (Utilities|FlowControl|Sequence
    (:then_0
      (Class|TYTestSpawnActor|Spin))))

(event EventBeginPlay
  ;[1 1 1] 사운드가 재생되고 있는 동안은 매 프레임 PlaybackPercentEvent 가 실행됩니다. PlaybackPercent(전체의 몇% 재생했는지)에 Duration(오디오의 길이)을 곱하는 것으로 현재의 재생 시간도 취득할 수 있습니다.
  (bind _output_get (Variables|Default|SetSoundDuration (Variables|/Script/Engine.SoundBase|GetDuration (Variables|Default|GetSoundWave))))
  (Components|Activation|Deactivate (Variables|Default|GetAudio1)))

(fn ConstructionScript)