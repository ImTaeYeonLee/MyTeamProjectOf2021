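; Test spawner Blueprint that repeatedly fires three circle-shot patterns on independent intervals.
; Tick runs a Sequence over three accumulating timers, each compared against its own CreateTime variable.
; When a timer reaches its threshold, it calls its matching CircleShot function and resets to zero.
; The shot functions' bodies are not part of these graphs, and BeginPlay, overlap and construction logic are empty.
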(event EventBeginPlay)

(event Collision|EventActorBeginOverlap
  (params (OtherActor :type Actor%20Object%20Reference)))

(event EventTick
  (params (DeltaSeconds :type Float%20%28single-precision%29))
  (Utilities|FlowControl|Sequence
    (:then_0
      (bind _output_get (Variables|Default|SetCurrentTime (+ DeltaSeconds (Variables|Default|GetCurrentTime))))
      (if (>= _output_get (Variables|Default|GetCreateTime))
        (Class|TYTestSpawnActor|CircleShot1)
        (Variables|Default|SetCurrentTime 0.0)))
    (:then_1
      (bind _output_get_2 (Variables|Default|SetCurrentTime2 (+ DeltaSeconds (Variables|Default|GetCurrentTime2))))
      (if (>= _output_get_2 (Variables|Default|GetCreateTime_2))
        (Class|TYTestSpawnActor|CircleShot2)
        (Variables|Default|SetCurrentTime2 0.0)))
    (:then_2
      (bind _output_get_3 (Variables|Default|SetCurrentTime3 (+ DeltaSeconds (Variables|Default|GetCurrentTime3))))
      (if (>= _output_get_3 (Variables|Default|GetCreateTime_3))
        (Class|TYTestSpawnActor|CircleShot3)
        (Variables|Default|SetCurrentTime3 0.0)))))

(fn ConstructionScript)