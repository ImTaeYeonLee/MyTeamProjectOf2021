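; Music-synced test actor that plays a SoundWave and calls Spin on audio onsets.
; BeginPlay binds the playback-percent callback, which converts progress to elapsed seconds and fetches channel-0 onset times and strengths once from OnsetNTR.
; Each callback fires Spin for at most one passed onset, then removes it from both arrays.
; Timed CircleShots, ConstantQ cube scaling and loudness- or strength-scaled BP_TY_RhythmRewardNode spawning remain disconnected; Tick is empty.
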(event Custom|PlaybackPercentEvent
  (params (PlayingSoundWave :type Sound%20Wave%20Object%20Reference) (PlaybackPercent :type Float%20%28single-precision%29))
  (bind _onsetntr (Variables|Default|GetOnsetNTR))
  (bind _soundduration (Variables|Default|GetSoundDuration))
  (bind (_outonsettimestamps _outonsetstrengths) (Class|OnsetNRT|GetChannelOnsetsBetweenTimes _onsetntr 0.0 _soundduration))
  (Variables|Default|SetPlayedTime (* PlaybackPercent (Variables|Default|GetSoundDuration)))
  (Utilities|FlowControl|Sequence
    (:then_0
      ;[1 1 1] Onset
      (Utilities|FlowControl|Sequence
        (:then_0
          (Utilities|FlowControl|DoOnce false
            (:Completed
              (Variables|Default|SetTimestamp _outonsettimestamps)
              (Variables|Default|SetStrength _outonsetstrengths))))
        (:then_1
          (bind (_array_element _array_index) (Utilities|Array|ForEachLoopwithBreak (Variables|Default|GetTimestamp) :!label _label)
            (:LoopBody
              (if (>= (Variables|Default|GetPlayedTime) _array_element)
                (Class|TYTestSpawnActor|Spin)
                (Utilities|Array|RemoveIndex (Variables|Default|GetTimestamp) _array_index)
                (Utilities|Array|RemoveIndex (Variables|Default|GetStrength) _array_index)
                (goto _label Break)))))))))

(event Collision|EventActorBeginOverlap
  (params (OtherActor :type Actor%20Object%20Reference)))

(event EventTick
  (params (DeltaSeconds :type Float%20%28single-precision%29)))

(event EventBeginPlay
  (bind _audio1 (Variables|Default|GetAudio1))
  ;[1 1 1] 사운드가 재생되고 있는 동안은 매 프레임 PlaybackPercentEvent 가 실행됩니다. PlaybackPercent(전체의 몇% 재생했는지)에 Duration(오디오의 길이)을 곱하는 것으로 현재의 재생 시간도 취득할 수 있습니다.
  (bind _output_get (Variables|Default|SetSoundDuration (Variables|/Script/Engine.SoundBase|GetDuration (Variables|Default|GetSoundWave))))
  (EventDispatchers|AssignOnAudioPlaybackPercent _audio1 (delegate Custom|PlaybackPercentEvent))
  (Audio|Components|Audio|SetSound _audio1 (Variables|Default|GetSoundWave))
  (Audio|Components|Audio|Play _audio1 0.0))

(fn ConstructionScript)