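; Test network player controller that handles pawn speed adjustment, an inventory toggle and voice chat registration.
; While right mouse is held, Tick adds half the wheel axis value to the possessed pawn's PlayerMove MoveSpeed, with a lower limit.
; The I key shows or hides an inventory widget created at BeginPlay, with animation and sound.
; On possess, after a short delay, it registers remote and local talkers and caches the PC pawn.
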(event EventBeginPlay
  ;[1 1 1] 인벤토리 생성
  (bind _returnvalue (UserInterface|CreateWidget "/Game/TY/UI/ItemInventory/Invectory.Invectory_C" self))
  (UserInterface|Viewport|AddtoPlayerScreen _returnvalue)
  (Widget|SetVisibility _returnvalue "Hidden"))

(event EventPossess
  (params (PossessedPawn :type Pawn%20Object%20Reference))
  (bind _self self)
  ;[1 1 1] 폰에 빙의하면
  (Utilities|FlowControl|Delay 0.5)
  (Utilities|FlowControl|Sequence
    (:then_0
      ;[1 1 1] IP가 다른 플레이어들도 보이스챗 사용자로 등록
      (Class|AdvancedVoiceLibrary|RegisterRemoteTalker (Class|AdvancedSessionsLibrary|GetUniqueNetID _self))
      (Class|AdvancedVoiceLibrary|RegisterLocalTalker (Math|Conversions|ToByte(Integer) (Class|GameplayStatics|GetPlayerControllerID _self))))
    (:then_1
      ;[1 1 1] PlayerPawn에 형변환한 대상을 CurrentPlayerPawn으로 정의, 타깃의 PlayerMoveComponent의 MoveSpeed(속도) 값을 가져온다.
      (bind _asbp_ty_test_network_player_pawn (Utilities|Casting|CastToBP_TY_Test_Network_PlayerPawn_PC PossessedPawn))
      (bind _output_get (Variables|Default|SetCurrentPlayerPawn _asbp_ty_test_network_player_pawn)))))

(event EventTick
  (params (DeltaSeconds :type Float%20%28single-precision%29))
  ;[1 1 1] 오른쪽 누른 상태일 때 true
  (if (Variables|Default|GetIsRightButtonPresseing)
    ;[1 1 1] 나온 값이 0.5보다 작거나 같다면, MoveSpeed를 0.5로 Set한다
    (if (>= (+ (/ (stale Input|MouseEvents|MouseWheelAxis AxisValue) 2.0) (Variables|/Script/UE_VtuberStudio.TY_PC_MoveActorComponent|GetmoveSpeed (Variables|/Script/UE_VtuberStudio.TY_PC_PlayerPawn|GetplayerMove (stale EventPossess _output_get)))) 0.5)
      (bind _output_get (Variables|/Script/UE_VtuberStudio.TY_PC_MoveActorComponent|SetmoveSpeed (Variables|/Script/UE_VtuberStudio.TY_PC_PlayerPawn|GetplayerMove (stale EventPossess _output_get)) (+ (/ (stale Input|MouseEvents|MouseWheelAxis AxisValue) 2.0) (Variables|/Script/UE_VtuberStudio.TY_PC_MoveActorComponent|GetmoveSpeed (Variables|/Script/UE_VtuberStudio.TY_PC_PlayerPawn|GetplayerMove (stale EventPossess _output_get))))))
      (Variables|Default|SetTempMoveSpeed _output_get)
      (Development|PrintString (Utilities|String|ToString(Float) _output_get))
      (else
        (bind _output_get_2 (Variables|/Script/UE_VtuberStudio.TY_PC_MoveActorComponent|SetmoveSpeed (Variables|/Script/UE_VtuberStudio.TY_PC_PlayerPawn|GetplayerMove (stale EventPossess _output_get)) 0.5))
        (Development|PrintString (Utilities|String|ToString(Float) _output_get_2))))))

(event Input|MouseEvents|MouseWheelAxis
  (params (AxisValue :type Float%20%28single-precision%29))
  ;[1 1 1] 나온 값이 0.5보다 작거나 같다면, MoveSpeed를 0.5로 Set한다
  (Variables|Default|SetMouse%20Wheel%20Axis%20Value AxisValue))

(event Input|KeyboardEvents|I
  (params (Key :type Key%20Structure))
  (:Pressed
    (if (Widget|IsVisible (stale EventBeginPlay _returnvalue))
      (Audio|PlaySound2D "/Game/InterfaceSound/Cue/018_MagicCard_Click_Cue.018_MagicCard_Click_Cue" 1.0 1.0 0.0 0 0)
      (UserInterface|Animation|PlayAnimation (stale EventBeginPlay _returnvalue) (Variables|/Game/TY/UI/ItemInventory/Invectory.Invectory_C|GetInventoryHiddenAnim_ (stale EventBeginPlay _returnvalue)) 0.0 1 "Forward" 1.0 false)
      (Utilities|FlowControl|Delay 0.5)
      ;[1 1 1] 코멘트
      (Widget|SetVisibility (stale EventBeginPlay _returnvalue) "Hidden")
      (else
        (Audio|PlaySound2D "/Game/InterfaceSound/Cue/018_MagicCard_Click_Cue.018_MagicCard_Click_Cue" 1.0 1.0 0.0 0 0)
        (UserInterface|Animation|PlayAnimation (stale EventBeginPlay _returnvalue) (Variables|/Game/TY/UI/ItemInventory/Invectory.Invectory_C|GetInventoryVisibleAnim_ (stale EventBeginPlay _returnvalue)) 0.0 1 "Forward" 1.0 false)
        (Widget|SetVisibility (stale EventBeginPlay _returnvalue) "Visible")))))

(event Input|KeyboardEvents|8
  (params (Key :type Key%20Structure)))

(event Input|MouseEvents|RightMouseButton
  (params (Key :type Key%20Structure))
  ;[1 1 1] 변수로 상태 제어
  (:Pressed
    (Variables|Default|SetIsRightButtonPresseing true)
    (Development|PrintString (Utilities|String|ToString(Boolean) (Variables|Default|GetIsRightButtonPresseing))))
  (:Released
    (Variables|Default|SetIsRightButtonPresseing false)))

(fn ConstructionScript)