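; PC player pawn for a network test, with photo mode, push-to-talk voice chat and screen fades; it hides both hands on BeginPlay.
; FlipFlop events toggle the photo-mode and viewer widgets; photo mode also swaps VR and photo cameras.
; While photo mode is on, movement, look, zoom, focus and reset input forward to its widget.
; Timelines drive the OBS camera plane's opacity through Tick, and TakeShotFade flashes the screen white.
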(event Custom|Remove%20PhotoMode%20Viewer%20Widget
  (bind _returnvalue (Game|GetPlayerController 0))
  (bind _returnvalue_2 (Game|GetPlayerController 0))
  ;[1 1 1] Photo Mode Events
  ;;[1 0.09759 0] Toggle Photo Mode Viewer
  (Utilities|FlowControl|FlipFlop
    (:A
      (bind _returnvalue_3 (UserInterface|CreateWidget "/Game/TY/UI/ScreenShot/PhotoMode_Viewer.PhotoMode_Viewer_C" (Game|GetPlayerController 0)))
      (bind _output_get (Variables|Default|SetPhotoModeViewer _returnvalue_3))
      (UserInterface|Viewport|AddtoViewport _output_get 0)
      (Input|SetInputModeGameandUI _returnvalue 0 "DoNotLock" false)
      (Variables|/Script/Engine.PlayerController|SetbShowMouseCursor _returnvalue true)
      ;;;[0 1 0.9947] 글로벌 시간 흐름 속도 제어
      (Utilities|Time|SetGlobalTimeDilation 1.0)
      (Variables|Default|SetIsPhotoModeViewerOn true))
    (:B
      (Widget|RemovefromParent (Variables|Default|GetPhotoModeViewer))
      (Input|SetInputModeGameandUI _returnvalue_2 0 "DoNotLock" false)
      (Variables|/Script/Engine.PlayerController|SetbShowMouseCursor _returnvalue_2 false)
      (Utilities|Time|SetGlobalTimeDilation 1.0)
      (Variables|Default|SetIsPhotoModeViewerOn false))))

(event Custom|Remove%20PhotoMode%20Widget
  (bind _returnvalue (Game|GetPlayerController 0))
  (bind _photomode_camera (Variables|Default|GetPhotoMode_Camera))
  ;[1 1 1] Photo Mode Events
  ;;[1 0.09759 0] Toggle Photo Mode
  (Utilities|FlowControl|FlipFlop
    (:A
      (bind _returnvalue_2 (UserInterface|CreateWidget "/Game/TY/UI/ScreenShot/PhotoMode_Widget.PhotoMode_Widget_C" (Game|GetPlayerController 0)))
      (bind _output_get (Variables|Default|SetPhotoModeUI _returnvalue_2))
      (UserInterface|Viewport|AddtoViewport _output_get 0)
      (Input|SetInputModeGameandUI _returnvalue 0 "DoNotLock" false)
      (Variables|/Script/Engine.PlayerController|SetbShowMouseCursor _returnvalue true)
      (Transformation|ResetRelativeTransform _photomode_camera)
      (Components|Activation|SetActive (Variables|Default|GetplayerCam_vr) false false)
      (Components|Activation|SetActive _photomode_camera true false)
      ;;;[0 0.9031 1] 글로벌 시간 흐름 제어
      (Utilities|Time|SetGlobalTimeDilation 1.0)
      (Variables|Default|SetIsPhotoModeOn true))
    (:B
      (Widget|RemovefromParent (Variables|Default|GetPhotoModeUI))
      (Input|SetInputModeGameandUI (Game|GetPlayerController 0) 0 "DoNotLock" false)
      (Components|Activation|SetActive (Variables|Default|GetplayerCam_vr) true false)
      (Components|Activation|SetActive (Variables|Default|GetPhotoMode_Camera) false false)
      (Default|ResetEffectSettings (Variables|Default|GetPhotoModeUI))
      (Variables|/Script/Engine.PlayerController|SetbShowMouseCursor (Game|GetPlayerController 0) false)
      (Utilities|Time|SetGlobalTimeDilation 1.0)
      (Variables|Default|SetIsPhotoModeOn false))))

(event Custom|TakeShotFade
  (bind _returnvalue (Game|GetPlayerCameraManager 0))
  (CameraFades|StartCameraFade _returnvalue 0.0 0.9 0.15 "(R=1.000000,G=1.000000,B=1.000000,A=1.000000)" false false)
  (Utilities|FlowControl|Delay 0.15)
  (CameraFades|StartCameraFade _returnvalue 0.9 0.0 0.15 "(R=1.000000,G=1.000000,B=1.000000,A=1.000000)" false false))

(event Custom|OBSCameraFadeOut
  ;[1 1 1] 어두워지기
  (bind _track (Timeline|타임라인_2 PlayFromStart)
    (:Update
      (Variables|Default|SetScalaValue _track))))

(event Custom|OBSCameraFadeIn
  ;[1 1 1] 밝아지기
  (bind _track (Timeline|타임라인_0 PlayFromStart)
    (:Update
      (Variables|Default|SetScalaValue _track))))

(event Custom|PhotoModeViewer_Start
  (bind _returnvalue (Game|GetPlayerController 0))
  (bind _returnvalue_2 (Game|GetPlayerController 0))
  ;[1 1 1] Photo Mode Events
  ;;[1 0.09759 0] Toggle Photo Mode Viewer
  (Utilities|FlowControl|FlipFlop
    (:A
      (bind _returnvalue_3 (UserInterface|CreateWidget "/Game/TY/UI/ScreenShot/PhotoMode_Viewer.PhotoMode_Viewer_C" (Game|GetPlayerController 0)))
      (bind _output_get (Variables|Default|SetPhotoModeViewer _returnvalue_3))
      (UserInterface|Viewport|AddtoViewport _output_get 0)
      (Input|SetInputModeGameandUI _returnvalue 0 "DoNotLock" false)
      (Variables|/Script/Engine.PlayerController|SetbShowMouseCursor _returnvalue true)
      ;;;[0 1 0.9947] 글로벌 시간 흐름 속도 제어
      (Utilities|Time|SetGlobalTimeDilation 1.0)
      (Variables|Default|SetIsPhotoModeViewerOn true))
    (:B
      (Widget|RemovefromParent (Variables|Default|GetPhotoModeViewer))
      (Input|SetInputModeGameandUI _returnvalue_2 0 "DoNotLock" false)
      (Variables|/Script/Engine.PlayerController|SetbShowMouseCursor _returnvalue_2 false)
      (Utilities|Time|SetGlobalTimeDilation 1.0)
      (Variables|Default|SetIsPhotoModeViewerOn false))))

(event Custom|PhotoMode_Start
  (bind _returnvalue (Game|GetPlayerController 0))
  (bind _photomode_camera (Variables|Default|GetPhotoMode_Camera))
  ;[1 1 1] Photo Mode Events
  ;;[1 0.09759 0] Toggle Photo Mode
  (Utilities|FlowControl|FlipFlop
    (:A
      (bind _returnvalue_2 (UserInterface|CreateWidget "/Game/TY/UI/ScreenShot/PhotoMode_Widget.PhotoMode_Widget_C" (Game|GetPlayerController 0)))
      (bind _output_get (Variables|Default|SetPhotoModeUI _returnvalue_2))
      (UserInterface|Viewport|AddtoViewport _output_get 0)
      (Input|SetInputModeGameandUI _returnvalue 0 "DoNotLock" false)
      (Variables|/Script/Engine.PlayerController|SetbShowMouseCursor _returnvalue true)
      (Transformation|ResetRelativeTransform _photomode_camera)
      (Components|Activation|SetActive (Variables|Default|GetplayerCam_vr) false false)
      (Components|Activation|SetActive _photomode_camera true false)
      ;;;[0 0.9031 1] 글로벌 시간 흐름 제어
      (Utilities|Time|SetGlobalTimeDilation 1.0)
      (Variables|Default|SetIsPhotoModeOn true))
    (:B
      (Widget|RemovefromParent (Variables|Default|GetPhotoModeUI))
      (Input|SetInputModeGameandUI (Game|GetPlayerController 0) 0 "DoNotLock" false)
      (Components|Activation|SetActive (Variables|Default|GetplayerCam_vr) true false)
      (Components|Activation|SetActive (Variables|Default|GetPhotoMode_Camera) false false)
      (Default|ResetEffectSettings (Variables|Default|GetPhotoModeUI))
      (Variables|/Script/Engine.PlayerController|SetbShowMouseCursor (Game|GetPlayerController 0) false)
      (Utilities|Time|SetGlobalTimeDilation 1.0)
      (Variables|Default|SetIsPhotoModeOn false))))

(event EventBeginPlay
  (bind _returnvalue (Rendering|Material|CreateDynamicMaterialInstance "/Game/TY/Effects/BlackFadeIn.BlackFadeIn" "None" "None" :!class /Script/Engine.KismetMaterialLibrary))
  (bind _output_get (Variables|Default|SetMaterial _returnvalue))
  (Rendering|Material|SetMaterial (Variables|Default|GetOBSCameraPlane) 0 _output_get)
  (Variables|Default|SetScalaValue 1.0)
  (Input|SetInputModeGameandUI (Game|GetPlayerController 0) 0 "DoNotLock" false)
  (Rendering|SetVisibility (Variables|Default|GetleftHand) false false))

(event Collision|EventActorBeginOverlap
  (params (OtherActor :type Actor%20Object%20Reference)))

(event EventPossessed
  (params (NewController :type Controller%20Object%20Reference))
  (Rendering|SetVisibility (Variables|Default|GetOBSCameraPlane) true false))

(event EventTick
  (params (DeltaSeconds :type Float%20%28single-precision%29))
  (Utilities|FlowControl|Sequence
    (:then_0
      (Rendering|Material|SetScalarParameterValue (Variables|Default|GetMaterial) "Oppacity" (Variables|Default|GetScalaValue) :!class /Script/Engine.MaterialInstanceDynamic))
    (:then_1)))

(event Input|ActionEvents|InputActionVoiceChat
  (params (Key :type Key%20Structure :default "None"))
  (bind _returnvalue (Class|GameplayStatics|GetPlayerControllerID))
  (:Pressed
    ;[1 1 1] 누르는 동안 이 플레이어 (콘트롤러)의 네트워크 보이스 챗 사용 가능
    (Class|AdvancedVoiceLibrary|StartNetworkedVoice (Math|Conversions|ToByte(Integer) _returnvalue))
    (Development|PrintString "Speaking"))
  (:Released
    ;[1 1 1] 릴리즈하면 사용 불가
    (Class|AdvancedVoiceLibrary|StopNetworkedVoice (Math|Conversions|ToByte(Integer) _returnvalue))
    (Development|PrintString "NotSpeaking" true true "(R=1.000000,G=0.000000,B=0.010689,A=1.000000)")))

(event Input|ActionEvents|InputActionPC_RotateReset
  (params (Key :type Key%20Structure :default "None"))
  ;[1 1 1] Photo Mode Events
  ;;[1 0.09759 0] Events
  (:Pressed
    (if (Variables|Default|GetIsPhotoModeOn)
      (Default|PhotoModeResetCamera (Variables|Default|GetPhotoModeUI)))))

(event Input|ActionEvents|InputActionFocus
  (params (Key :type Key%20Structure :default "None"))
  ;[1 1 1] Photo Mode Events
  ;;[1 0.09759 0] Events
  (:Pressed
    (if (Variables|Default|GetIsPhotoModeOn)
      (Default|PhotoModeFocusCamera (Variables|Default|GetPhotoModeUI)))))

(event Input|AxisEvents|InputAxisPC_ZoomInWheel
  (params (AxisValue :type Float%20%28single-precision%29))
  ;[1 1 1] Photo Mode Events
  ;;[1 0.09759 0] Events
  (if (Variables|Default|GetIsPhotoModeOn)
    (Default|PhotoModeZoom (Variables|Default|GetPhotoModeUI) AxisValue)))

(event Input|AxisEvents|InputAxisMoveForward
  (params (AxisValue :type Float%20%28single-precision%29))
  ;[1 1 1] Photo Mode Events
  ;;[1 0.09759 0] Events
  (if (Variables|Default|GetIsPhotoModeOn)
    (Default|PhotoModeMoveForward (Variables|Default|GetPhotoModeUI) AxisValue)))

(event Input|AxisEvents|InputAxisMoveRight
  (params (AxisValue :type Float%20%28single-precision%29))
  ;[1 1 1] Photo Mode Events
  ;;[1 0.09759 0] Events
  (if (Variables|Default|GetIsPhotoModeOn)
    (Default|PhotoModeMoveRight (Variables|Default|GetPhotoModeUI) AxisValue)))

(event Input|AxisEvents|InputAxisPC_MoveVertical
  (params (AxisValue :type Float%20%28single-precision%29))
  ;[1 1 1] Photo Mode Events
  ;;[1 0.09759 0] Events
  (if (Variables|Default|GetIsPhotoModeOn)
    (Default|PhotoModeMoveUp (Variables|Default|GetPhotoModeUI) AxisValue)))

(event Input|AxisEvents|InputAxisTurn
  (params (AxisValue :type Float%20%28single-precision%29))
  ;[1 1 1] Photo Mode Events
  ;;[1 0.09759 0] Events
  (if (Variables|Default|GetIsPhotoModeOn)
    (Default|PhotoModeRotateYaw (Variables|Default|GetPhotoModeUI) AxisValue)))

(event Input|AxisEvents|InputAxisLookUp
  (params (AxisValue :type Float%20%28single-precision%29))
  ;[1 1 1] Photo Mode Events
  ;;[1 0.09759 0] Events
  (if (Variables|Default|GetIsPhotoModeOn)
    (Default|PhotoModeRotatePitch (Variables|Default|GetPhotoModeUI) AxisValue)))

(fn ConstructionScript)